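; BP_BreakSpawner repeatedly spawns random breakable actors using its spawn areas.
; On BeginPlay it registers itself as spawner on each SpawnArea, then loops every two seconds, asking a spawn object for a random position and breakable class.
; Each spawned actor attaches to the spawner; the loop stops on a zero position or non-Actor class.
; AttachChildren is an empty stub, and DeleteWithDelay is unused in this graph.
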(event EventBeginPlay
  (CallFunction|AttachChildren)
  (CallFunction|AssignSpawner)
  (Components|StaticMesh|SetStaticMesh (Variables|Default|GetTest) 0)
  (bind _returnvalue (Class|SpawnBreakables|GetSpawnObject :!label _label))
  (bind _returnvalue_2 (Class|SpawnArea|RandomPos _returnvalue))
  (if (Class|KismetMathLibrary|NotEqualExactlyVectorVector _returnvalue_2 "0, 0, 0")
    (bind _returnvalue_3 (Class|SpawnArea|RandomBreakable _returnvalue))
    (bind _asactor (Utilities|Casting|CastToActorClass _returnvalue_3)
      (:then
        (bind _returnvalue_4 (Game|SpawnActorfromClass _asactor (Math|Conversions|ToTransform(Vector) _returnvalue_2) "Undefined" "MultiplyWithRoot" 0 0))
        (Transformation|AttachActorToActor _returnvalue_4 self "None" "KeepRelative" "KeepRelative" "KeepRelative" true)
        (Utilities|FlowControl|Delay 2.0)
        (goto _label))
      (:CastFailed
        (Development|PrintString "Non-Actor in array")))))

(fn ConstructionScript)

(fn AssignSpawner
  (for _array_element (Variables|Default|GetspawnAreas)
    (Variables|/Script/ChaosTruck.SpawnArea|Setspawner _array_element self)))

(fn AttachChildren)