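; Breakable traffic cone that gets launched upward when a truck hits it.
; When its Box is overlapped, it checks that HasGivenPoints is false and that the other component's owner, or that owner's owner, is a BP_Truck.
; It then applies a large upward force to every static mesh component on the cone.
; The graph only reads HasGivenPoints, and a node to disable mesh collision is left unconnected.
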(event OnComponentBeginOverlap(Box)
  (params (OverlappedComponent :type Primitive%20Component%20Object%20Reference) (OtherActor :type Actor%20Object%20Reference) (OtherComp :type Primitive%20Component%20Object%20Reference) (OtherBodyIndex :type Integer) (bFromSweep :type Boolean) (SweepResult :type Hit%20Result%20Structure%20%28by%20ref%29))
  (bind _returnvalue (Components|GetOwner OtherComp))
  (if (not (Variables|Default|GethasGivenPoints))
    (Utilities|Casting|CastToBP_Truck _returnvalue
      (:then
        _)
      (:CastFailed
        (Utilities|Casting|CastToBP_Truck (Components|GetOwner _returnvalue))))
    (for _array_element (Actor|GetComponentsByClass "/Script/Engine.StaticMeshComponent")
      (bind _asstatic_mesh_component (Utilities|Casting|CastToStaticMeshComponent _array_element))
      (Physics|AddForce _asstatic_mesh_component "0.000000,0.000000,500000.000000" "None" false))))

(event EventBeginPlay)

(event Collision|EventActorBeginOverlap
  (params (OtherActor :type Actor%20Object%20Reference)))

(fn ConstructionScript)