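; Breakable prop that shatters on overlap and awards the truck player score and boost once.
; Box overlap wakes its Geometry Collection, if present, triggers a child master field to break it, and plays audio.
; The server awards points, plays controller rumble and starts delayed hiding; clients add boost immediately to avoid lag.
; The respawn delay leads nowhere, as the Respawn call and flag reset are unwired.
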(event OnComponentBeginOverlap(Box)
  (params (OverlappedComponent :type Primitive%20Component%20Object%20Reference) (OtherActor :type Actor%20Object%20Reference) (OtherComp :type Primitive%20Component%20Object%20Reference) (OtherBodyIndex :type Integer) (bFromSweep :type Boolean) (SweepResult :type Hit%20Result%20Structure%20%28by%20ref%29))
  (bind _self self)
  (bind _uthething (Variables|/Script/ChaosTruck.Breakable|GetUtheThing _self))
  ;[0.15 0.15 0.15 0.5] Handles the visuals of the destrutible so mostly the geometry collection and audio
  (bind _asbp_master_field (Utilities|Casting|CastToBP_MasterField (Variables|/Script/Engine.ChildActorComponent|GetChildActor (Variables|Default|GetBP_MasterField))))
  (Utilities|IsValid _uthething
    (:Is%20Valid
      (bind _asgeometry_collection_component (Utilities|Casting|CastToGeometryCollectionComponent _uthething)
        (:then
          (Class|PrimitiveComponent|WakeRigidBody _asgeometry_collection_component "None")
          (Default|TriggerBreak _asbp_master_field))
        (:CastFailed
          _))
      (Audio|Components|Audio|Play (Variables|Default|GetBreakingAudio) 0.0)
      (if (not (Variables|Default|GethasGivenPoints))
        (Variables|Default|SethasGivenPoints true)
        (CallFunction|AddtoPlayer OtherComp)))))

(event Custom|Delete
  (bind _self self)
  (bind _uthething (Variables|/Script/ChaosTruck.Breakable|GetUtheThing _self))
  ;[0.15 0.15 0.15 0.5] Destruction and respawning code
  (Utilities|FlowControl|Delay (Variables|Default|GettimetoDestroy))
  (if (Utilities|IsValid (Variables|/Script/ChaosTruck.Breakable|GetUtheThing self))
    (Rendering|SetVisibility _uthething false false)
    (bind _asgeometry_collection_component (Utilities|Casting|CastToGeometryCollectionComponent _uthething)
      (:then
        (Class|PrimitiveComponent|PutRigidBodytoSleep _asgeometry_collection_component "None"))
      (:CastFailed
        (bind _asstatic_mesh_component (Utilities|Casting|CastToStaticMeshComponent _uthething))
        (Class|PrimitiveComponent|PutRigidBodytoSleep _asstatic_mesh_component "None")))
    (Utilities|FlowControl|Delay (Variables|Default|GetrespawnTime))
    (else
      (Development|PrintString "Not Valid!!" true true "(R=1.000000,G=0.094932,B=0.000000,A=1.000000)" 1e+01))))

(event Custom|addToPlayer
  (params (Other :type Actor%20Component%20Object%20Reference))
  (bind _returnvalue (Components|GetOwner Other))
  ;[0.15 0.15 0.15 0.5] Adding points and Boost and da rumble
  (bind _asbp_truck (Utilities|Casting|CastToBP_Truck _returnvalue)
    (:then
      (Variables|Default|SetPlayer%20State (Variables|/Script/Engine.Pawn|GetPlayerState _asbp_truck))
      (bind _asbp_truck_player_state (Utilities|Casting|CastToBP_TruckPlayerState (Variables|Default|GetPlayer%20State) :!label _label))
      (Variables|Default|SetPlayer%20State 0)
      (Networking|SwitchHasAuthority
        (:Authority
          (Game|Feedback|ClientPlayForceFeedback (Game|GetPlayerController _asbp_truck_player_state) "/Game/Input/FF_Breakable.FF_Breakable" "None" false false false)
          (Default|AddScore _asbp_truck_player_state (Variables|Default|GetScoreValue))
          (Default|AddBoost _asbp_truck_player_state (Variables|Default|GetBoostValue))
          (CallFunction|Delete))
        (:Remote
          ;;[0.15 0.15 0.15 0.5] This is so the clients don't have a delay to added boost
          (Variables|/Game/Blueprints/Players/CustomTruck/BP_TruckPlayerState.BP_TruckPlayerState_C|SetBoostNum _asbp_truck_player_state (+ (Variables|/Game/Blueprints/Players/CustomTruck/BP_TruckPlayerState.BP_TruckPlayerState_C|GetBoostNum _asbp_truck_player_state) (Variables|Default|GetBoostValue))))))
    (:CastFailed
      ;;[0.15 0.15 0.15 0.5] Sometimes it grabs the shell and not the truck this is for that
      (bind _asbp_truck_2 (Utilities|Casting|CastToBP_Truck (Components|GetOwner _returnvalue))
        (:then
          (Variables|Default|SetPlayer%20State (Variables|/Script/Engine.Pawn|GetPlayerState _asbp_truck_2))
          (goto _label))
        (:CastFailed
          (Development|PrintString "A Non Truck Has broke a breakable"))))))

(event EventBeginPlay
  (bind _returnvalue (Actor|GetComponentbyClass "/Script/GeometryCollectionEngine.GeometryCollectionComponent"))
  (bind _returnvalue_2 (Actor|GetComponentbyClass "/Script/Engine.StaticMeshComponent"))
  (bind _self self)
  ;[0.15 0.15 0.15 0.5] Logic for getting gemetry collectiosn or meshes based on the breakable on start (used for respawning)
  (Variables|Default|SetStartPos (Transformation|GetActorTransform self))
  (if (Utilities|IsValid _returnvalue)
    (Variables|/Script/ChaosTruck.Breakable|SetUtheThing _self _returnvalue)
    (elif (Utilities|IsValid _returnvalue_2)
      (Variables|/Script/ChaosTruck.Breakable|SetUtheThing _self _returnvalue_2)
      (else
        (Development|PrintString "No Applicable mesh for the breakable")))))

(fn ConstructionScript)

(fn BreakEvent
  (params (Piece :type Primitive%20Component%20Object%20Reference) (index :type Integer) (GeometryCollection :type Geometry%20Collection%20Component%20Object%20Reference))
  (bind _hitvelocity (Variables|Default|GetHitVelocity))
  (Physics|SetEnableGravity Piece true)
  (Class|GeometryCollectionComponent|ApplyLinearVelocity GeometryCollection index _hitvelocity)
  (if (== index 1)
    (Class|GeometryCollectionComponent|ApplyLinearVelocity GeometryCollection 3 _hitvelocity)))

(fn BreakEventNew
  (params (Other :type Actor%20Component%20Object%20Reference))
  (Networking|SwitchHasAuthority))