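; BP_BreakableShip is a destructible ghost ship that shatters section by section as trigger boxes are overlapped.
; Each box pairs with a BP_MasterField child actor and passes both to a shared BreakPart event.
; BreakPart wakes the ship's Geometry Collection, triggers that field's break, then destroys the field component and box so each section breaks only once.
; The overlap events apply no check on the overlapping actor.
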(event OnComponentBeginOverlap(Box1)
  (params (OverlappedComponent :type Primitive%20Component%20Object%20Reference) (OtherActor :type Actor%20Object%20Reference) (OtherComp :type Primitive%20Component%20Object%20Reference) (OtherBodyIndex :type Integer) (bFromSweep :type Boolean) (SweepResult :type Hit%20Result%20Structure%20%28by%20ref%29))
  (CallFunction|BreakPart (Variables|Default|GetBP_MasterField) (Variables|Default|GetBox1)))

(event OnComponentBeginOverlap(Box9)
  (params (OverlappedComponent :type Primitive%20Component%20Object%20Reference) (OtherActor :type Actor%20Object%20Reference) (OtherComp :type Primitive%20Component%20Object%20Reference) (OtherBodyIndex :type Integer) (bFromSweep :type Boolean) (SweepResult :type Hit%20Result%20Structure%20%28by%20ref%29))
  (CallFunction|BreakPart (Variables|Default|GetChildActor7) (Variables|Default|GetBox9)))

(event OnComponentBeginOverlap(Box12)
  (params (OverlappedComponent :type Primitive%20Component%20Object%20Reference) (OtherActor :type Actor%20Object%20Reference) (OtherComp :type Primitive%20Component%20Object%20Reference) (OtherBodyIndex :type Integer) (bFromSweep :type Boolean) (SweepResult :type Hit%20Result%20Structure%20%28by%20ref%29))
  (CallFunction|BreakPart (Variables|Default|GetChildActor10) (Variables|Default|GetBox12)))

(event OnComponentBeginOverlap(Box8)
  (params (OverlappedComponent :type Primitive%20Component%20Object%20Reference) (OtherActor :type Actor%20Object%20Reference) (OtherComp :type Primitive%20Component%20Object%20Reference) (OtherBodyIndex :type Integer) (bFromSweep :type Boolean) (SweepResult :type Hit%20Result%20Structure%20%28by%20ref%29))
  (CallFunction|BreakPart (Variables|Default|GetChildActor6) (Variables|Default|GetBox8)))

(event OnComponentBeginOverlap(Box2)
  (params (OverlappedComponent :type Primitive%20Component%20Object%20Reference) (OtherActor :type Actor%20Object%20Reference) (OtherComp :type Primitive%20Component%20Object%20Reference) (OtherBodyIndex :type Integer) (bFromSweep :type Boolean) (SweepResult :type Hit%20Result%20Structure%20%28by%20ref%29))
  (CallFunction|BreakPart (Variables|Default|GetChildActor) (Variables|Default|GetBox2)))

(event OnComponentBeginOverlap(Box3)
  (params (OverlappedComponent :type Primitive%20Component%20Object%20Reference) (OtherActor :type Actor%20Object%20Reference) (OtherComp :type Primitive%20Component%20Object%20Reference) (OtherBodyIndex :type Integer) (bFromSweep :type Boolean) (SweepResult :type Hit%20Result%20Structure%20%28by%20ref%29))
  (CallFunction|BreakPart (Variables|Default|GetChildActor1) (Variables|Default|GetBox3)))

(event OnComponentBeginOverlap(Box4)
  (params (OverlappedComponent :type Primitive%20Component%20Object%20Reference) (OtherActor :type Actor%20Object%20Reference) (OtherComp :type Primitive%20Component%20Object%20Reference) (OtherBodyIndex :type Integer) (bFromSweep :type Boolean) (SweepResult :type Hit%20Result%20Structure%20%28by%20ref%29))
  (CallFunction|BreakPart (Variables|Default|GetChildActor2) (Variables|Default|GetBox4)))

(event OnComponentBeginOverlap(Box5)
  (params (OverlappedComponent :type Primitive%20Component%20Object%20Reference) (OtherActor :type Actor%20Object%20Reference) (OtherComp :type Primitive%20Component%20Object%20Reference) (OtherBodyIndex :type Integer) (bFromSweep :type Boolean) (SweepResult :type Hit%20Result%20Structure%20%28by%20ref%29))
  (CallFunction|BreakPart (Variables|Default|GetChildActor3) (Variables|Default|GetBox5)))

(event OnComponentBeginOverlap(Box6)
  (params (OverlappedComponent :type Primitive%20Component%20Object%20Reference) (OtherActor :type Actor%20Object%20Reference) (OtherComp :type Primitive%20Component%20Object%20Reference) (OtherBodyIndex :type Integer) (bFromSweep :type Boolean) (SweepResult :type Hit%20Result%20Structure%20%28by%20ref%29))
  (CallFunction|BreakPart (Variables|Default|GetChildActor4) (Variables|Default|GetBox6)))

(event OnComponentBeginOverlap(Box7)
  (params (OverlappedComponent :type Primitive%20Component%20Object%20Reference) (OtherActor :type Actor%20Object%20Reference) (OtherComp :type Primitive%20Component%20Object%20Reference) (OtherBodyIndex :type Integer) (bFromSweep :type Boolean) (SweepResult :type Hit%20Result%20Structure%20%28by%20ref%29))
  (CallFunction|BreakPart (Variables|Default|GetChildActor5) (Variables|Default|GetBox7)))

(event OnComponentBeginOverlap(Box11)
  (params (OverlappedComponent :type Primitive%20Component%20Object%20Reference) (OtherActor :type Actor%20Object%20Reference) (OtherComp :type Primitive%20Component%20Object%20Reference) (OtherBodyIndex :type Integer) (bFromSweep :type Boolean) (SweepResult :type Hit%20Result%20Structure%20%28by%20ref%29))
  (CallFunction|BreakPart (Variables|Default|GetChildActor9) (Variables|Default|GetBox11)))

(event OnComponentBeginOverlap(Box10)
  (params (OverlappedComponent :type Primitive%20Component%20Object%20Reference) (OtherActor :type Actor%20Object%20Reference) (OtherComp :type Primitive%20Component%20Object%20Reference) (OtherBodyIndex :type Integer) (bFromSweep :type Boolean) (SweepResult :type Hit%20Result%20Structure%20%28by%20ref%29))
  (CallFunction|BreakPart (Variables|Default|GetChildActor8) (Variables|Default|GetBox10)))

(event Custom|BreakPart
  (params (MasterField :type Child%20Actor%20Component%20Object%20Reference) (BoxCollider :type Box%20Component%20Object%20Reference))
  ;[0.15 0.15 0.15 0.5] General Event For Breaking parts
  (bind _asbp_master_field (Utilities|Casting|CastToBP_MasterField (Variables|/Script/Engine.ChildActorComponent|GetChildActor MasterField)))
  (Class|PrimitiveComponent|WakeRigidBody (Variables|Default|GetGC_SM_GhostShip) "None")
  (Default|TriggerBreak _asbp_master_field)
  (Components|DestroyComponent MasterField)
  (Components|DestroyComponent BoxCollider))

(fn ConstructionScript)