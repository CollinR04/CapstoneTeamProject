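; Breakable land mine built on a geometry collection that blows apart when it fractures.
; Each Chaos break event turns on gravity for the broken component and flings that piece outward from the actor root with a strong fixed linear velocity.
; Separately, any overlap with the box destroys the weak boost pad component.
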(event OnComponentBeginOverlap(Box)
  (params (OverlappedComponent :type Primitive%20Component%20Object%20Reference) (OtherActor :type Actor%20Object%20Reference) (OtherComp :type Primitive%20Component%20Object%20Reference) (OtherBodyIndex :type Integer) (bFromSweep :type Boolean) (SweepResult :type Hit%20Result%20Structure%20%28by%20ref%29))
  (Components|DestroyComponent (Variables|Default|GetBP_boostPad_Weak)))

(event OnChaosBreakEvent(GC_SM_Destructable_WaterMine_2)
  (params (BreakEvent :type Chaos%20Break%20Event%20Structure%20%28by%20ref%29))
  (bind (_component _location _orientation _velocity _angularvelocity _extents _mass _index) (Utilities|Struct|BreakChaosBreakEvent BreakEvent))
  ;[0.15 0.15 0.15 0.5] My main goal is blow up
  (Physics|SetEnableGravity _component true)
  (Class|GeometryCollectionComponent|ApplyLinearVelocity (Variables|Default|GetGC_SM_Destructable_WaterMine_2) _index (* (Math|Vector|Normalize (- _location (Transformation|GetWorldLocation (Variables|Default|GetDefaultSceneRoot)))) 1e+04)))

(event EventBeginPlay)

(fn ConstructionScript)