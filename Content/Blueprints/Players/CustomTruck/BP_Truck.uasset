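; Networked player truck pawn with socketed suspension wheels, health, an armor shell, and collision, hazard and damage feedback.
; On BeginPlay it looks up the player's character in DT_PlayerInfo to set wheel materials, boost and fire-trail effects, replicated via server and multicast events.
; The server spawns and attaches the character's BP_Shell, whose notifies drive truck damage and armor state; health changes are broadcast through a dispatcher.
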(event Custom|TakeDamageFeedback
  (Game|Feedback|ClientPlayForceFeedback (Game|GetPlayerController 0) "/Game/Input/FF_Damage.FF_Damage" "None" false false false))

(event Custom|ArmorDamageFeedback
  (Game|Feedback|ClientPlayForceFeedback (Game|GetPlayerController 0) "/Game/Input/FF_ArmorBreak.FF_ArmorBreak" "None" false false false))

(event Custom|BreakableFeedback
  (Game|Feedback|ClientPlayForceFeedback (Game|GetPlayerController 0) 0 "None" false false false))

(event EventTick
  (params (DeltaSeconds :type Float%20%28single-precision%29)))

(event EventBeginPlay
  (bind _self self)
  ;[0.15 0.15 0.15 0.5] Grab all suspensions
  (Variables|Default|SetSuspension (Actor|GetComponentsByClass "/Game/Blueprints/Players/CustomTruck/BP_TruckSuspension.BP_TruckSuspension_C"))
  (Utilities|FlowControl|Delay 0.5) ; makes sure we are possessed before doing anything
  (bind _asbp_truck_player_controller (Utilities|Casting|CastToBP_TruckPlayerController (Components|GetOwner)))
  (Variables|/Game/Blueprints/Players/CustomTruck/BP_TruckPlayerController.BP_TruckPlayerController_C|SetRepName _asbp_truck_player_controller "")
  (bind _asbp_truck_player_state (Utilities|Casting|CastToBP_TruckPlayerState (Variables|/Script/Engine.Controller|GetPlayerState _asbp_truck_player_controller)))
  (bind _returnvalue (Utilities|GetDataTableRow "/Game/UI/DT_PlayerInfo.DT_PlayerInfo" (Utilities|String|StringToName (Variables|/Game/Blueprints/Players/CustomTruck/BP_TruckPlayerState.BP_TruckPlayerState_C|GetCharacterName _asbp_truck_player_state)))
    (:then
      (CallFunction|SetWheels (.characterwheel _returnvalue))
      (CallFunction|SetBoost _self _asbp_truck_player_state)
      (CallFunction|SetFireTrail _self _asbp_truck_player_state)
      (Networking|SwitchHasAuthority
        (:Authority
          (CallFunction|ServerCreateShell self _asbp_truck_player_controller _asbp_truck_player_state))))))

(event OnComponentBeginOverlap(CollisionDetection)
  (params (OverlappedComponent :type Primitive%20Component%20Object%20Reference) (OtherActor :type Actor%20Object%20Reference) (OtherComp :type Primitive%20Component%20Object%20Reference) (OtherBodyIndex :type Integer) (bFromSweep :type Boolean) (SweepResult :type Hit%20Result%20Structure%20%28by%20ref%29))
  (bind _asbp_pickup (Utilities|Casting|CastToBP_Pickup OtherActor)
    (:CastFailed
      (bind _ashazard (Utilities|Casting|CastToHazard OtherActor))
      (Default|HazardCollision (Variables|Default|GetBP_HazardComponent1) self _ashazard))))

(event OnComponentEndOverlap(CollisionDetection)
  (params (OverlappedComponent :type Primitive%20Component%20Object%20Reference) (OtherActor :type Actor%20Object%20Reference) (OtherComp :type Primitive%20Component%20Object%20Reference) (OtherBodyIndex :type Integer))
  (bind _asbp_fire_actor (Utilities|Casting|CastToBP_FireActor OtherActor))
  (Default|FireTickDamageEnd (Variables|Default|GetBP_HazardComponent1) self _asbp_fire_actor))

(event OnComponentBeginOverlap(BodyCollision)
  (params (OverlappedComponent :type Primitive%20Component%20Object%20Reference) (OtherActor :type Actor%20Object%20Reference) (OtherComp :type Primitive%20Component%20Object%20Reference) (OtherBodyIndex :type Integer) (bFromSweep :type Boolean) (SweepResult :type Hit%20Result%20Structure%20%28by%20ref%29))
  (Utilities|Casting|CastToBP_Pickup OtherActor
    (:CastFailed
      (Utilities|Casting|CastToHazard OtherActor
        (:CastFailed
          (Utilities|Casting|CastToBP_Breakable OtherActor
            (:CastFailed
              (bind _asbp_truck (Utilities|Casting|CastToBP_Truck OtherActor)
                (:then
                  (if (not (== _asbp_truck self))
                    (Audio|Components|Audio|Play (Variables|Default|GetCollisionAudio) 0.0 :!label _label)
                    (CallFunction|BreakableFeedback)))
                (:CastFailed
                  (Utilities|Casting|CastToBP_Shell OtherActor
                    (:CastFailed
                      (goto _label))))))))))))

(event Custom|ReplicateRibbonDeactivate
  (params (Ribbon :type Niagara%20Component%20Object%20Reference))
  (CallFunction|DeactivateonAllClients Ribbon))

(event Custom|DeactivateOnAllClients
  (params (Ribbon :type Niagara%20Component%20Object%20Reference))
  (Components|Activation|Deactivate Ribbon))

(event Custom|TempOffAllClients
  (params (Ribbon :type Niagara%20Component%20Object%20Reference))
  (Niagara|SetNiagaraVariable(Float) Ribbon "UserSpawnRate" 0.0))

(event Custom|ActivateOnAllClients
  (params (Ribbon :type Niagara%20Component%20Object%20Reference))
  (Components|Activation|SetActive Ribbon true false))

(event Custom|ReplicateTempOn
  (params (Ribbon :type Niagara%20Component%20Object%20Reference))
  (CallFunction|TemponAllClients Ribbon))

(event Custom|ReplicateRibbonActivate
  (params (Ribbon :type Niagara%20Component%20Object%20Reference))
  (CallFunction|ActivateonAllClients Ribbon))

(event Custom|ReplicateTempOff
  (params (Ribbon :type Niagara%20Component%20Object%20Reference))
  (CallFunction|TempOffAllClients Ribbon))

(event Custom|TempOnAllClients
  (params (Ribbon :type Niagara%20Component%20Object%20Reference))
  (bind _result (Math|Integer|IncrementInt (Variables|Default|GetFireID))
    (:%20%20
      (Class|NiagaraComponent|SetNiagaraVariableInt Ribbon "UserID" _result)
      (Niagara|SetNiagaraVariable(Float) Ribbon "UserSpawnRate" 4e+02))))

(event Custom|TruckCollisionDamage
  (params (Damage :type Float%20%28double-precision%29) (OtherActor :type Actor%20Object%20Reference))
  (Development|PrintString "calling take damage on truck")
  (CallFunction|TakeDamage Damage OtherActor))

(event Custom|Blowup
  (CallFunction|ServerBlowup))

(event Custom|Server_Blowup
  (CallFunction|SelfDestruct))

(event Custom|CheckCollectionsEmpty
  (params (bIsEmpty :type Boolean))
  (if bIsEmpty
    (bind _result (Math|Integer|IncrementInt (Variables|Default|GetNumEmptyCollections))
      (:%20%20
        (if (>= _result (Utilities|Array|Length (Variables|Default|GetArmorCollections)))
          (Variables|Default|SetbHasArmor false))))))

(event Custom|Server_CreateShell
  (params (Truck :type BP%20Truck%20Object%20Reference) (Controller :type Controller%20Object%20Reference) (PlayerState :type BP%20Truck%20Player%20State%20Object%20Reference))
  (bind _returnvalue (Utilities|GetDataTableRow "/Game/UI/DT_PlayerInfo.DT_PlayerInfo" (Utilities|String|StringToName (Variables|/Game/Blueprints/Players/CustomTruck/BP_TruckPlayerState.BP_TruckPlayerState_C|GetCharacterName PlayerState)))
    (:then
      (bind _returnvalue_2 (Game|SpawnActorfromClass (.charactershell _returnvalue) (Transformation|GetActorTransform Truck) "AdjustIfPossibleButAlwaysSpawn" "MultiplyWithRoot" Truck Truck))
      (bind _asbp_shell (Utilities|Casting|CastToBP_Shell _returnvalue_2))
      (Variables|Default|SetShell _asbp_shell)
      (Transformation|AttachComponentToComponent (Variables|Default|GetShell) (Variables|Default|GetChasis) "Shell" "SnapToTarget" "SnapToTarget" "SnapToTarget" true)
      (Transformation|AddRelativeRotation (Variables|/Game/Blueprints/Armor/BP_Shell.BP_Shell_C|GetDefaultSceneRoot (Variables|Default|GetShell)) "0.000000,-90.000000,0.000000" false false)
      ;[0.15 0.15 0.15 0.5] Bind truck collisions to cause damage
      (EventDispatchers|BindEventtoOnTruckDamageNotify (Variables|Default|GetShell) (EventDispatchers|CreateEvent :!event Custom|TruckCollisionDamage))
      ;[0.15 0.15 0.15 0.5] Bind for having armor checks
      (EventDispatchers|BindEventtoOnCollectionEmptyNotify (Variables|Default|GetShell) (EventDispatchers|CreateEvent :!event Custom|CheckCollectionsEmpty))
      (EventDispatchers|BindEventtoOnArmorBreakNotify (Variables|Default|GetShell) (EventDispatchers|CreateEvent :!event Custom|ArmorBreakEvent))
      ;[0.15 0.15 0.15 0.5] Set the speed at which the armor gains shield
      (bind _output_get (Variables|Default|SetShieldSpeedThreshold (* (Variables|Default|GetPercentForShield) (Variables|/Script/ChaosTruck.TruckMovementComponent|GetBaseMaxSpeed (Variables|Default|GetMovementComponent)))))
      (Default|SetSpeedThreshold (Variables|Default|GetShell) _output_get))))

(event Custom|Server_DestroyShell
  (params (Truck :type Actor%20Object%20Reference))
  (bind _shell (Variables|Default|GetShell))
  (Utilities|IsValid Truck
    (:Is%20Valid
      (Utilities|IsValid _shell
        (:Is%20Valid
          (Actor|DestroyActor _shell))))))

(event EventEndPlay
  (params (EndPlayReason :type EEndPlayReason%20Enum :default "Destroyed"))
  (Networking|SwitchHasAuthority
    (:Authority
      (CallFunction|ServerDestroyShell self))))

(event Custom|ArmorBreakEvent
  (params (BrokenArmor :type Armor%20Object%20Reference))
  (Audio|Components|Audio|Play (Variables|Default|GetArmorBreak1) 0.0)
  (Game|Feedback|ClientStartCameraShake (Game|GetPlayerController 0) "/Game/Blueprints/VFX/BP_ShakeDamaged.BP_ShakeDamaged_C" 1.0 "World" "0, 0, 0")
  (CallFunction|ArmorDamageFeedback))

(event Custom|Server_SetBoost
  (params (Truck :type BP%20Truck%20Object%20Reference) (PlayerState :type BP%20Truck%20Player%20State%20Object%20Reference))
  (CallFunction|MulticastSetBoost Truck PlayerState))

(event Custom|Multicast_SetBoost
  (params (Truck :type BP%20Truck%20Object%20Reference) (Player%20State :type BP%20Truck%20Player%20State%20Object%20Reference))
  (bind _ps_yellow_boost (Variables|BP_Truck_C|GetPS_Yellow_Boost Truck))
  (bind _ps_yellow_boost1 (Variables|BP_Truck_C|GetPS_Yellow_Boost1 Truck))
  (bind _returnvalue (Utilities|GetDataTableRow "/Game/UI/DT_PlayerInfo.DT_PlayerInfo" (Utilities|String|StringToName (Variables|/Game/Blueprints/Players/CustomTruck/BP_TruckPlayerState.BP_TruckPlayerState_C|GetCharacterName Player%20State)))
    (:then
      (Class|NiagaraComponent|SetAsset _ps_yellow_boost (.characterboost _returnvalue) true)
      (Transformation|SetRelativeLocation _ps_yellow_boost (.rightboostpos _returnvalue) false true)
      (Class|NiagaraComponent|SetAsset _ps_yellow_boost1 (.characterboost _returnvalue) true)
      (Transformation|SetRelativeLocation _ps_yellow_boost1 (.leftboostpos _returnvalue) false true))))

(event Custom|SetBoost
  (params (Truck :type BP%20Truck%20Object%20Reference) (Player%20State :type BP%20Truck%20Player%20State%20Object%20Reference))
  (Networking|SwitchHasAuthority
    (:Authority
      (Utilities|FlowControl|Delay 1.0)
      (CallFunction|MulticastSetBoost Truck Player%20State))
    (:Remote
      (CallFunction|ServerSetBoost Truck Player%20State))))

(event Custom|Multicast_ActivateBoost
  (params (bActive :type Boolean))
  (Components|Activation|SetActive (Variables|Default|GetPS_Yellow_Boost) bActive false)
  (Components|Activation|SetActive (Variables|Default|GetPS_Yellow_Boost1) bActive false))

(event Custom|ActivateBoost
  (params (bActive :type Boolean))
  (Networking|SwitchHasAuthority
    (:Authority
      (CallFunction|MulticastActivateBoost bActive))
    (:Remote
      (CallFunction|ServerActivateBoost bActive))))

(event Custom|Server_ActivateBoost
  (params (bActive :type Boolean))
  (CallFunction|MulticastActivateBoost bActive))

(event Custom|SetWheels
  (params (Mesh :type Static%20Mesh%20Object%20Reference))
  (Networking|SwitchHasAuthority
    (:Authority
      (CallFunction|ChangeWheelMesh Mesh))
    (:Remote
      (CallFunction|ServerSetWheels Mesh))))

(event Custom|Multicast_SetWheels
  (params (Mesh :type Static%20Mesh%20Object%20Reference)))

(event Custom|Server_SetWheels
  (params (Mesh :type Static%20Mesh%20Object%20Reference))
  (CallFunction|ChangeWheelMesh Mesh))

(event Custom|Server_SetFireTrail
  (params (Truck :type BP%20Truck%20Object%20Reference) (PlayerState :type BP%20Truck%20Player%20State%20Object%20Reference))
  (CallFunction|MulticastSetFireTrail Truck PlayerState))

(event Custom|MulticastSetFireTrail
  (params (Truck :type BP%20Truck%20Object%20Reference) (Player%20State :type BP%20Truck%20Player%20State%20Object%20Reference))
  (bind _returnvalue (Utilities|GetDataTableRow "/Game/UI/DT_PlayerInfo.DT_PlayerInfo" (Utilities|String|StringToName (Variables|/Game/Blueprints/Players/CustomTruck/BP_TruckPlayerState.BP_TruckPlayerState_C|GetCharacterName Player%20State)))
    (:then
      (Class|NiagaraComponent|SetAsset (Variables|BP_Truck_C|GetPS_Fire_Trail1 Truck) (.characterfire _returnvalue) true)
      (Class|NiagaraComponent|SetAsset (Variables|BP_Truck_C|GetPS_Fire_Trail2 Truck) (.characterfire _returnvalue) true))))

(event Custom|SetFireTrail
  (params (Truck :type BP%20Truck%20Object%20Reference) (Player%20State :type BP%20Truck%20Player%20State%20Object%20Reference))
  (Networking|SwitchHasAuthority
    (:Authority
      (Utilities|FlowControl|Delay 1.0)
      (CallFunction|MulticastSetFireTrail Truck Player%20State))
    (:Remote
      (CallFunction|ServerSetFireTrail Truck Player%20State))))

(fn ConstructionScript
  ;[0.15 0.15 0.15 0.5] Attach wheels to sockets on Chasis
  (CallFunction|AttachWheels)
  ;[0.15 0.15 0.15 0.5] Reset var on creation
  (Variables|Default|SetbHasArmor true))

(fn TakeDamage
  (params (Damage :type Float%20%28double-precision%29) (OtherActor :type Actor%20Object%20Reference))
  (bind _output_get (Variables|Default|SetTruckHealth (- (Variables|Default|GetTruckHealth) Damage)))
  (Development|PrintString (Utilities|String|ToString(Float) _output_get))
  (Audio|Components|Audio|Play (Variables|Default|GetDamageAudio) 0.0)
  (bind _asbp_truck_player_controller (Utilities|Casting|CastToBP_TruckPlayerController (Pawn|GetController)))
  (Default|CallOnHealthChange _output_get (Variables|Default|GetMaxHealth) _asbp_truck_player_controller OtherActor)
  (Game|Feedback|ClientStartCameraShake _asbp_truck_player_controller "/Game/Blueprints/VFX/BP_ShakeDamaged.BP_ShakeDamaged_C" 1.0 "World" "0, 0, 0")
  (CallFunction|TakeDamageFeedback))

(fn OnRepRepID)

(fn OnRepRepName
  (Default|CallOnPowerUpPickup (Variables|Default|GetRepID) (Variables|Default|GetRepName)))

(fn AttachWheels
  (bind _bp_wheelgrandma3 (Variables|Default|GetBP_WheelGrandma3))
  (bind _bp_wheelgrandma2 (Variables|Default|GetBP_WheelGrandma2))
  (bind _bp_wheelgrandma1 (Variables|Default|GetBP_WheelGrandma1))
  (bind _bp_wheelgrandma (Variables|Default|GetBP_WheelGrandma))
  (Variables|/Game/Blueprints/Players/CustomTruck/BP_SuspensionWheel.BP_SuspensionWheel_C|SetSuspension _bp_wheelgrandma (Variables|Default|GetBL_Suspension))
  (Transformation|AttachComponentToComponent _bp_wheelgrandma (Variables|Default|GetChasis) "BL_Wheel" "KeepRelative" "KeepRelative" "KeepRelative" true)
  (Variables|/Game/Blueprints/Players/CustomTruck/BP_SuspensionWheel.BP_SuspensionWheel_C|SetSuspension _bp_wheelgrandma1 (Variables|Default|GetBR_Suspension))
  (Transformation|AttachComponentToComponent _bp_wheelgrandma1 (Variables|Default|GetChasis) "BR_Wheel" "KeepRelative" "KeepRelative" "KeepRelative" true)
  (Variables|/Game/Blueprints/Players/CustomTruck/BP_SuspensionWheel.BP_SuspensionWheel_C|SetSuspension _bp_wheelgrandma3 (Variables|Default|GetFL_Suspension))
  (Transformation|AttachComponentToComponent _bp_wheelgrandma3 (Variables|Default|GetChasis) "FL_Wheel" "KeepRelative" "KeepRelative" "KeepRelative" true)
  (Variables|/Game/Blueprints/Players/CustomTruck/BP_SuspensionWheel.BP_SuspensionWheel_C|SetSuspension _bp_wheelgrandma2 (Variables|Default|GetFR_Suspension))
  (Transformation|AttachComponentToComponent _bp_wheelgrandma2 (Variables|Default|GetChasis) "FR_Wheel" "KeepRelative" "KeepRelative" "KeepRelative" true))

(fn ChangeWheelMesh
  (params (Mesh :type Static%20Mesh%20Object%20Reference))
  (bind _bp_wheelgrandma2 (Variables|Default|GetBP_WheelGrandma2))
  (bind _bp_wheelgrandma3 (Variables|Default|GetBP_WheelGrandma3))
  (bind _bp_wheelgrandma1 (Variables|Default|GetBP_WheelGrandma1))
  (bind _bp_wheelgrandma (Variables|Default|GetBP_WheelGrandma))
  (Variables|/Game/Blueprints/Players/CustomTruck/BP_SuspensionWheel.BP_SuspensionWheel_C|SetMat0 _bp_wheelgrandma (Rendering|Material|GetMaterial Mesh 0))
  (Variables|/Game/Blueprints/Players/CustomTruck/BP_SuspensionWheel.BP_SuspensionWheel_C|SetMat1 _bp_wheelgrandma (Rendering|Material|GetMaterial Mesh 1))
  (Variables|/Game/Blueprints/Players/CustomTruck/BP_SuspensionWheel.BP_SuspensionWheel_C|SetMat0 _bp_wheelgrandma1 (Rendering|Material|GetMaterial Mesh 0))
  (Variables|/Game/Blueprints/Players/CustomTruck/BP_SuspensionWheel.BP_SuspensionWheel_C|SetMat1 _bp_wheelgrandma1 (Rendering|Material|GetMaterial Mesh 1))
  (Variables|/Game/Blueprints/Players/CustomTruck/BP_SuspensionWheel.BP_SuspensionWheel_C|SetMat0 _bp_wheelgrandma2 (Rendering|Material|GetMaterial Mesh 0))
  (Variables|/Game/Blueprints/Players/CustomTruck/BP_SuspensionWheel.BP_SuspensionWheel_C|SetMat1 _bp_wheelgrandma2 (Rendering|Material|GetMaterial Mesh 1))
  (Variables|/Game/Blueprints/Players/CustomTruck/BP_SuspensionWheel.BP_SuspensionWheel_C|SetMat0 _bp_wheelgrandma3 (Rendering|Material|GetMaterial Mesh 0))
  (Variables|/Game/Blueprints/Players/CustomTruck/BP_SuspensionWheel.BP_SuspensionWheel_C|SetMat1 _bp_wheelgrandma3 (Rendering|Material|GetMaterial Mesh 1)))

(fn SelfDestruct
  (bind _output_get (Variables|Default|SetTruckHealth 0.0))
  (bind _asbp_truck_player_controller (Utilities|Casting|CastToBP_TruckPlayerController (Pawn|GetController)))
  (Default|CallOnHealthChange _output_get (Variables|Default|GetMaxHealth) _asbp_truck_player_controller))