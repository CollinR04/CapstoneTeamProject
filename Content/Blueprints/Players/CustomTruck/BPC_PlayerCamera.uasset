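; Player camera component that drives the truck's spring arm for look, auto-recentering, zoom and boost effects.
; Look input rotates the arm using saved sensitivity, and a timer-counted idle delay lets it interpolate back while grounded and upright.
; When airborne and flipped or spinning, the arm switches to absolute rotation aligned with velocity yaw, set only once at low speed.
; Boost adds speed-line post-processing, and arm length steps with boost and throttle flags.
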(event EventBeginPlay
  (bind _asbp_truck (Utilities|Casting|CastToBP_Truck (Components|GetOwner)))
  (Variables|Default|SetPlayer _asbp_truck)
  (Variables|Default|SetTruckSpringArm (Variables|/Game/Blueprints/Players/CustomTruck/BP_Truck.BP_Truck_C|GetCamera_SpringArm _asbp_truck))
  (bind _asbp_truck_player_controller (Utilities|Casting|CastToBP_TruckPlayerController (Game|GetPlayerController 0)))
  (EventDispatchers|BindEventtoOnSpeedChange _asbp_truck_player_controller (EventDispatchers|CreateEvent :!event Custom|ChangeCameraDist))
  (bind _returnvalue (SaveGame|LoadGamefromSlot "settings"))
  (bind _asbp_settings_save_game (Utilities|Casting|CastToBP_Settings_SaveGame _returnvalue))
  (Variables|Default|SetCamera%20Sensitivity (Variables|/Game/Blueprints/UI/BP_Settings_SaveGame.BP_Settings_SaveGame_C|GetCameraSensitivity _asbp_settings_save_game))
  (Utilities|FlowControl|Delay 2.1)
  (Variables|Default|SetOriginal%20camera%20rotation (Transformation|GetWorldRotation (Variables|Default|GetTruckSpringArm))))

(event EventTick
  (params (DeltaSeconds :type Float%20%28single-precision%29))
  (CallFunction|ChangeCameraDist false false)
  (CallFunction|InterpstoOriginalRotation)
  (CallFunction|VelocityBasedCamera))

(event Custom|InterpsToOriginalRotation
  (bind _returnvalue (Utilities|Time|GetWorldDeltaSeconds))
  (bind _truckspringarm (Variables|Default|GetTruckSpringArm))
  (bind _truckspringarm_2 (Variables|Default|GetTruckSpringArm))
  (bind _relativerotation (Variables|/Script/Engine.SceneComponent|GetRelativeRotation _truckspringarm))
  (bind _returnvalue_2 (Math|Interpolation|FInterpTo (.pitch _relativerotation) -25.0 _returnvalue 1e+02))
  ;[0.15 0.15 0.15 0.5] Camera Auto Correction
  (bind _isupsidedown (CallFunction|CheckUpsideDown))
  (if (not _isupsidedown)
    (bind _asbp_truck_player_controller (Utilities|Casting|CastToBP_TruckPlayerController (Game|GetPlayerController 0)))
    (bind _bisonground (Default|CheckonGround _asbp_truck_player_controller))
    (if _bisonground
      (if (> (Variables|Default|GetInterping%20Timer%20Count) (Variables|Default|GetInterping%20Threshold))
        (if (not (Variables|Default|GetLooking))
          (if (> (.yaw _relativerotation) 0.0)
            ;;[0.15 0.15 0.15 0.5] Rotate left (less than 180)
            (Transformation|SetRelativeRotation _truckspringarm_2 (Math|Rotator|MakeRotator 0.0 _returnvalue_2 (Math|Interpolation|FInterpTo (.yaw _relativerotation) 0.0 (Utilities|Time|GetWorldDeltaSeconds) (Variables|Default|GetInterp%20Speed))) false false)
            (else
              ;;[0.15 0.15 0.15 0.5] Rotate right (more than 180)
              (Transformation|SetRelativeRotation _truckspringarm_2 (Math|Rotator|MakeRotator 0.0 _returnvalue_2 (Math|Interpolation|FInterpTo (.yaw _relativerotation) 0.0 (Utilities|Time|GetWorldDeltaSeconds) (Variables|Default|GetInterp%20Speed))) false false))))
        (else
          ;;[0.15 0.15 0.15 0.5] Correction Delay
          (Utilities|FlowControl|DoOnce false
            (:Completed
              (Utilities|Time|SetTimerbyEvent (delegate Custom|AddDelayTime) (Variables|Default|GetInterping%20Count%20Speed) true))))))))

(event Custom|AddDelayTime
  (bind _interping_timer_count (Variables|Default|GetInterping%20Timer%20Count))
  ;[0.15 0.15 0.15 0.5] Camera Auto Correction
  ;;[0.15 0.15 0.15 0.5] Correction Delay
  (if (not (== _interping_timer_count (+ (Variables|Default|GetInterping%20Threshold) 1)))
    (Math|Integer|IncrementInt _interping_timer_count
      (:%20%20
        (Utilities|FlowControl|DoOnce false) ; enters at Reset
      ))))

(event Custom|VelocityBasedCamera
  (bind _truckspringarm (Variables|Default|GetTruckSpringArm))
  (bind _truckspringarm_2 (Variables|Default|GetTruckSpringArm))
  ;[0.15 0.15 0.15 0.5] Camera Follows velocity when in air
  (bind _asbp_truck_player_controller (Utilities|Casting|CastToBP_TruckPlayerController (Game|GetPlayerController 0)))
  (bind _bisonground (Default|CheckonGround _asbp_truck_player_controller))
  (bind _isupsidedown (CallFunction|CheckUpsideDown))
  (if (and (or _isupsidedown (> (Math|Vector|VectorLength (Physics|GetPhysicsAngularVelocityinDegrees (Variables|/Script/ChaosTruck.Truck|GetChasis (Variables|/Game/Blueprints/Players/CustomTruck/BP_TruckPlayerController.BP_TruckPlayerController_C|GetTruck _asbp_truck_player_controller)) "None")) 1e+01)) (not _bisonground))
    (bind _returnvalue (Physics|GetPhysicsLinearVelocity (Variables|/Script/ChaosTruck.Truck|GetChasis (Variables|/Game/Blueprints/Players/CustomTruck/BP_TruckPlayerController.BP_TruckPlayerController_C|GetTruck _asbp_truck_player_controller)) "None")) ; Must be upside down or spinning, and wheels not on ground
    (if (< (Math|Vector|VectorLength _returnvalue) 1.2e+03)
      ;;[0.15 0.15 0.15 0.5] Upside down (or spinning), wheels not on the ground but we think the car is going slow enough that it's on the ground and needs to be flipped
      (Variables|/Script/Engine.SceneComponent|SetbAbsoluteRotation _truckspringarm true)
      (Utilities|FlowControl|DoOnce false :!label _label
        (:Completed
          (Transformation|SetWorldRotation _truckspringarm (Math|Rotator|CombineRotators "-25.000000,0.000000,0.000000" (Math|Rotator|MakeRotator 0.0 0.0 (.Yaw (Math|Rotator|BreakRotator (Math|Rotator|MakeRotfromX (Transformation|GetVelocity (Variables|/Game/Blueprints/Players/CustomTruck/BP_TruckPlayerController.BP_TruckPlayerController_C|GetTruck _asbp_truck_player_controller))))))) false false)))
      (else
        ;;[0.15 0.15 0.15 0.5] Upside down (or spinning), wheels not on the ground; going fast enough we think it's in the air
        (Variables|/Script/Engine.SceneComponent|SetbAbsoluteRotation _truckspringarm_2 true)
        (Transformation|SetWorldRotation _truckspringarm_2 (Math|Rotator|CombineRotators "-25.000000,0.000000,0.000000" (Math|Rotator|MakeRotator 0.0 0.0 (.Yaw (Math|Rotator|BreakRotator (Math|Rotator|MakeRotfromX (Transformation|GetVelocity (Variables|/Game/Blueprints/Players/CustomTruck/BP_TruckPlayerController.BP_TruckPlayerController_C|GetTruck _asbp_truck_player_controller))))))) false false)))
    (else
      (Variables|/Script/Engine.SceneComponent|SetbAbsoluteRotation _truckspringarm_2 false)
      (goto _label Reset))))

(event Input|EnhancedActionEvents|EnhancedInputActionIA_Look
  (params (ActionValue :type Vector%202D%20Structure) (ElapsedSeconds :type Float%20%28double-precision%29) (TriggeredSeconds :type Float%20%28double-precision%29) (InputAction :type Input%20Action%20Object%20Reference :default "/Game/Input/IA_Look.IA_Look"))
  (bind _truckspringarm (Variables|Default|GetTruckSpringArm))
  (bind _truckspringarm_2 (Variables|Default|GetTruckSpringArm))
  (bind _truckspringarm_3 (Variables|Default|GetTruckSpringArm))
  (bind _relativerotation (Variables|/Script/Engine.SceneComponent|GetRelativeRotation _truckspringarm_2))
  (bind _relativerotation_2 (Variables|/Script/Engine.SceneComponent|GetRelativeRotation _truckspringarm))
  (bind (_roll _pitch _yaw) (Math|Rotator|BreakRotator _relativerotation))
  (bind (_roll_2 _pitch_2 _yaw_2) (Math|Rotator|BreakRotator _relativerotation_2))
  (bind _returnvalue (+ 3.6e+02 _yaw))
  (bind _returnvalue_2 (Math|Float|%(Float) _returnvalue 3.6e+02))
  ;[0.15 0.15 0.15 0.5] Camera Controls
  (:Triggered
    (Variables|Default|SetInterping%20Timer%20Count 0)
    (Variables|Default|SetLooking true)
    (Utilities|FlowControl|Sequence
      (:then_0
        ;;[0.15 0.15 0.15 0.5] Bound left/right looking to 80 - 280
        (if (or (> _returnvalue_2 2.8e+02) (< _returnvalue_2 8e+01))
          _
          (else
            _))
        (Transformation|AddRelativeRotation _truckspringarm_3 (Math|Rotator|MakeRotator 0.0 0.0 (* (.x ActionValue) (Variables|Default|GetCamera%20Sensitivity))) false false))
      (:then_1
        ;;[0.15 0.15 0.15 0.5] Bound up/down looking to (-25) - 25
        (if (or (> _pitch 25.1) (< _pitch -25.1))
          (Transformation|SetRelativeRotation _truckspringarm (Math|Rotator|MakeRotator _roll_2 (Math|Conversions|ToFloat(Integer) (Math|Float|Truncate _pitch_2)) _yaw_2) false false)
          (else
            (Transformation|AddRelativeRotation _truckspringarm_3 (Math|Rotator|MakeRotator 0.0 (* (.y ActionValue) (Variables|Default|GetCamera%20Sensitivity)) 0.0) false false))))))
  (:Completed
    (Variables|Default|SetLooking false)))

(event Custom|ChangeCameraDist
  (params (Boosting :type Boolean) (Throttling :type Boolean))
  (bind _truckspringarm (Variables|Default|GetTruckSpringArm))
  (bind _truckspringarm_2 (Variables|Default|GetTruckSpringArm))
  ;[0.15 0.15 0.15 0.5] Camera Zooming at speeds
  (if Boosting
    ;;[0.15 0.15 0.15 0.5] Change with boost
    (if (< (Variables|/Script/Engine.SpringArmComponent|GetTargetArmLength _truckspringarm) (Variables|Default|GetBoost%20Distance))
      (Variables|/Script/Engine.SpringArmComponent|SetTargetArmLength (Variables|Default|GetTruckSpringArm) (+ (Variables|/Script/Engine.SpringArmComponent|GetTargetArmLength _truckspringarm) (Variables|Default|GetBoost%20Zoom%20Speed))))
    (else
      ;;[0.15 0.15 0.15 0.5] Change with throttle
      (if Throttling
        (if (< (Variables|/Script/Engine.SpringArmComponent|GetTargetArmLength _truckspringarm) (Variables|Default|GetThrottle%20Max%20Distance))
          (Variables|/Script/Engine.SpringArmComponent|SetTargetArmLength _truckspringarm_2 (+ (Variables|/Script/Engine.SpringArmComponent|GetTargetArmLength _truckspringarm) (Variables|Default|GetCamera%20Zoom%20Out))))
        (elif (> (Variables|/Script/Engine.SpringArmComponent|GetTargetArmLength _truckspringarm) (Variables|Default|GetThrottle%20Min%20Distance))
          (Variables|/Script/Engine.SpringArmComponent|SetTargetArmLength _truckspringarm_2 (- (Variables|/Script/Engine.SpringArmComponent|GetTargetArmLength _truckspringarm) (Variables|Default|GetCamera%20Zoom%20In))))))))

(event Input|EnhancedActionEvents|EnhancedInputActionIA_Boost
  (params (ActionValue :type Boolean) (ElapsedSeconds :type Float%20%28double-precision%29) (TriggeredSeconds :type Float%20%28double-precision%29) (InputAction :type Input%20Action%20Object%20Reference :default "/Game/Input/IA_Boost.IA_Boost"))
  (bind _player (Variables|Default|GetPlayer))
  (bind _camera (Variables|/Game/Blueprints/Players/CustomTruck/BP_Truck.BP_Truck_C|GetCamera _player))
  ;[0.15 0.15 0.15 0.5] Speed Lines
  (:Triggered
    (bind _asbp_truck_player_state (Utilities|Casting|CastToBP_TruckPlayerState (Game|GetPlayerState 0)))
    (if (> (Variables|/Game/Blueprints/Players/CustomTruck/BP_TruckPlayerState.BP_TruckPlayerState_C|GetBoostNum _asbp_truck_player_state) 0.0)
      (bind _returnvalue (Rendering|Material|CreateDynamicMaterialInstance "/Game/VFX/VFXMaterials/M_ActionLines.M_ActionLines" "None" "None" :!class /Script/Engine.KismetMaterialLibrary))
      (Variables|/Script/Engine.CameraComponent|SetPostProcessSettings _camera (Utilities|Struct|MakePostProcessSettings (Utilities|Struct|MakeWeightedBlendables (Utilities|Array|MakeArray (Utilities|Struct|MakeWeightedBlendable 1.0 _returnvalue)))))
      (Class|CameraComponent|SetPostProcessBlendWeight _camera 1.0)
      (else
        (Utilities|FlowControl|Delay (Variables|Default|GetSpeedLineEndDelay) :!label _label)
        (Class|CameraComponent|SetPostProcessBlendWeight (Variables|/Game/Blueprints/Players/CustomTruck/BP_Truck.BP_Truck_C|GetCamera (Variables|Default|GetPlayer)) 0.0))))
  (:Completed
    (goto _label)))

(fn CheckUpsideDown
  (bind _asbp_truck_player_controller (Utilities|Casting|CastToBP_TruckPlayerController (Game|GetPlayerController 0)))
  (Utilities|IsValid (Variables|/Game/Blueprints/Players/CustomTruck/BP_TruckPlayerController.BP_TruckPlayerController_C|GetTruck _asbp_truck_player_controller)
    (:Is%20Valid
      (return (< (Math|Vector|DotProduct (Transformation|GetActorUpVector (Variables|/Game/Blueprints/Players/CustomTruck/BP_TruckPlayerController.BP_TruckPlayerController_C|GetTruck _asbp_truck_player_controller)) "0.000000,0.000000,1.000000") (Variables|Default|GetCamera%20Flip%20Angle))))))