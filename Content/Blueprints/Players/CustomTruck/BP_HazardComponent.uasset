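; Truck component that applies hazard effects on the server when an unarmored truck collides with another owner's hazard.
; Chains deal damage unless already exploded and temporarily cut max speed with a replicated ribbon effect.
; Overlapping fire actors are counted, dealing an initial hit and a looping timer tick until the count reaches zero.
; Other hazards deal one hit, with DoOnce gates plus delays throttling both chain and generic hits.
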(event Custom|FireTickDamage
  (bind _truck (Variables|Default|GetTruck))
  ;[0.15 0.15 0.15 0.5] Fire tick damage start
  (Networking|SwitchHasAuthority
    (:Authority
      (Utilities|IsValid _truck
        (:Is%20Valid
          (Default|TakeDamage _truck (Variables|/Script/ChaosTruck.Hazard|GetSecondDamage (stale Custom|HazardCollision _asbp_fire_actor)) (Variables|Default|GetOtherTruck)))
        (:Is%20Not%20Valid
          (Utilities|Time|ClearTimerbyFunctionName 0 "FireTickDamage"))))))

(event Custom|HazardCollision
  (params (TruckActor :type Actor%20Object%20Reference) (HazardActor :type Actor%20Object%20Reference))
  (Networking|SwitchHasAuthority
    (:Authority
      (bind _asbp_truck (Utilities|Casting|CastToBP_Truck TruckActor))
      (bind _output_get (Variables|Default|SetTruck _asbp_truck))
      (bind _ashazard (Utilities|Casting|CastToHazard HazardActor))
      (Variables|Default|SetOtherTruck (Components|GetOwner _ashazard))
      (if (not (Variables|/Game/Blueprints/Players/CustomTruck/BP_Truck.BP_Truck_C|GetbHasArmor _output_get))
        (if (not (== (Components|GetOwner _ashazard) TruckActor))
          (bind _asbp_chain (Utilities|Casting|CastToBP_Chain _ashazard)
            (:then
              (Utilities|FlowControl|DoOnce false :!label _label
                (:Completed
                  (Default|ReplicateRibbonActivate (Variables|Default|GetTruck) (Variables|/Game/Blueprints/Players/CustomTruck/BP_Truck.BP_Truck_C|GetSlowdown%20Chains (Variables|Default|GetTruck)))
                  (if (Variables|/Game/VFX/ParticleSystems/BP_Chain.BP_Chain_C|GetHasExploded _asbp_chain)
                    _
                    (else
                      (Default|TakeDamage (Variables|Default|GetTruck) (Variables|/Script/ChaosTruck.Hazard|GetSecondDamage _ashazard) (Variables|Default|GetOtherTruck))))
                  (Variables|/Game/Blueprints/Players/CustomTruck/BP_Truck.BP_Truck_C|SetMaxSpeed (Variables|Default|GetTruck) 0.5)
                  (Development|PrintString "hit by bomb")
                  (Utilities|FlowControl|Delay 1e+01)
                  (Variables|/Game/Blueprints/Players/CustomTruck/BP_Truck.BP_Truck_C|SetMaxSpeed (Variables|Default|GetTruck) 1.0)
                  (Default|ReplicateRibbonDeactivate (Variables|Default|GetTruck) (Variables|/Game/Blueprints/Players/CustomTruck/BP_Truck.BP_Truck_C|GetSlowdown%20Chains (Variables|Default|GetTruck)))
                  (goto _label Reset))))
            (:CastFailed
              (bind _asbp_fire_actor (Utilities|Casting|CastToBP_FireActor _ashazard)
                (:then
                  (Variables|Default|SetFireOverlapping (+ (Variables|Default|GetFireOverlapping) 1))
                  (if (== (Variables|Default|GetFireOverlapping) 1)
                    (Default|TakeDamage (Variables|Default|GetTruck) (Variables|/Script/ChaosTruck.Hazard|GetDamage _ashazard) (Variables|Default|GetOtherTruck))
                    (Utilities|Time|SetTimerbyFunctionName 0 "FireTickDamage" (Variables|/Script/ChaosTruck.Hazard|GetDamageInterval _asbp_fire_actor) true)))
                (:CastFailed
                  (Utilities|FlowControl|DoOnce false :!label _label_2
                    (:Completed
                      (Default|TakeDamage (Variables|Default|GetTruck) (Variables|/Script/ChaosTruck.Hazard|GetDamage _ashazard) (Variables|Default|GetOtherTruck))
                      (Utilities|FlowControl|Delay 0.7)
                      (goto _label_2 Reset))))))))))))

(event Custom|FireTickDamageEnd
  (params (TruckActor :type Actor%20Object%20Reference) (FireActor :type Actor%20Object%20Reference))
  ;[0.15 0.15 0.15 0.5] Fire tick damage end
  (Utilities|Casting|CastToBP_Truck TruckActor)
  (Utilities|Casting|CastToBP_FireActor FireActor)
  (Variables|Default|SetFireOverlapping (- (Variables|Default|GetFireOverlapping) 1))
  (if (== (Variables|Default|GetFireOverlapping) 0)
    (Utilities|Time|ClearTimerbyFunctionName 0 "FireTickDamage")))

(event EventBeginPlay)

(event EventTick
  (params (DeltaSeconds :type Float%20%28single-precision%29)))