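; Player state for truck players, holding boost, score, team and character identity.
; Boost additions cap at 100, and score additions record the latest gain with a short timer to reset it.
; Team replication recolors the truck's spotlight and cone, polling with delays until the truck pawn exists and exactly four pawns are present.
; CopyProperties carries character name and picture to the new state, and a server event sets the name.
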(event Custom|AddBoost
  (params (Amount :type Float%20%28double-precision%29))
  (bind _self self)
  ;[0.15 0.15 0.15 0.5] Adding Boost
  (if (< (+ (Variables|BP_TruckPlayerState_C|GetBoostNum _self) Amount) 1e+02)
    (Variables|BP_TruckPlayerState_C|SetBoostNum _self (+ (Variables|BP_TruckPlayerState_C|GetBoostNum _self) Amount))
    (else
      (Variables|BP_TruckPlayerState_C|SetBoostNum _self 1e+02))))

(event Custom|AddScore
  (params (Amount :type Integer))
  (bind _self self)
  ;[0.15 0.15 0.15 0.5] Adding Score
  (Utilities|Time|ClearTimerbyFunctionName 0 "BP_TruckPlayerState_AutoGenFunc")
  (Variables|BP_TruckPlayerState_C|SetPlayerScore _self (+ (Variables|BP_TruckPlayerState_C|GetPlayerScore _self) Amount))
  (Variables|Default|SetLastScoreIncrease Amount)
  (Utilities|Time|SetTimerbyEvent (EventDispatchers|CreateEvent :!event BPTruckPlayerStateAutoGenFunc) 1.0))

(event Custom|ChangeSpotLightColorReplicated
  ;[0.15 0.15 0.15 0.5] Change Spotlight Color based on team
  (bind _asbp_truck (Utilities|Casting|CastToBP_Truck (PlayerState|GetPawn self) :!label _label)
    (:then
      (if (== (Variables|Default|GetTeamID) 2)
        (Rendering|Components|Light|SetLightColor (Variables|/Game/Blueprints/Players/CustomTruck/BP_Truck.BP_Truck_C|GetSpotLight _asbp_truck) "(R=0.208637,G=0.074214,B=1.000000,A=1.000000)" true)
        (Rendering|Material|SetMaterial (Variables|/Game/Blueprints/Players/CustomTruck/BP_Truck.BP_Truck_C|GetSM_Light_Cone_Wide _asbp_truck) 0 "/Game/Materials/lightMaterials/Materials/M_ChildEmissive1_Inst.M_ChildEmissive1_Inst")
        (else
          (Rendering|Components|Light|SetLightColor (Variables|/Game/Blueprints/Players/CustomTruck/BP_Truck.BP_Truck_C|GetSpotLight _asbp_truck) "(R=1.000000,G=0.039546,B=0.000000,A=1.000000)" true)
          (Rendering|Material|SetMaterial (Variables|/Game/Blueprints/Players/CustomTruck/BP_Truck.BP_Truck_C|GetSM_Light_Cone_Wide _asbp_truck) 0 "/Game/Materials/lightMaterials/Materials/M_ChildEmissive1_InstRed.M_ChildEmissive1_InstRed"))))
    (:CastFailed
      (Utilities|FlowControl|Delay 0.2)
      (goto _label))))

(event Custom|ChangeSpotlightColorState
  ;[0.15 0.15 0.15 0.5] If Team ID is changed then they tell the Truck to change its spotlight Color
  (Utilities|Casting|CastToBP_Truck (PlayerState|GetPawn self) :!label _label
    (:then
      (bind _outactors (Actor|GetAllActorsOfClass "/Script/Engine.Pawn" :!label _label_2))
      (if (== (Utilities|Array|Length _outactors) 4)
        (CallFunction|ChangeSpotLightColorReplicated)
        (else
          (Utilities|FlowControl|Delay 0.2)
          (goto _label_2))))
    (:CastFailed
      (Utilities|FlowControl|Delay 0.2)
      (goto _label))))

(event EventRepTeamID
  ;[0.15 0.15 0.15 0.5] If Team ID is changed then they tell the Truck to change its spotlight Color
  (CallFunction|ChangeSpotlightColorState))

(event EventCopyProperties
  (params (NewPlayerState :type Player%20State%20Object%20Reference))
  (bind _asbp_truck_player_state (Utilities|Casting|CastToBP_TruckPlayerState NewPlayerState))
  (Variables|BP_TruckPlayerState_C|SetCharacterName _asbp_truck_player_state (Variables|Default|GetCharacterName))
  (Variables|BP_TruckPlayerState_C|SetCharacterPicture _asbp_truck_player_state (Variables|Default|GetCharacterPicture))
  (Development|PrintString "copying playerr state"))

(event Custom|SetCharName
  (params (PlayerState :type BP%20Truck%20Player%20State%20Object%20Reference) (CharacterName :type String))
  (CallFunction|ServerSetCharacterName PlayerState PlayerState CharacterName))

(event Custom|Server_SetCharacterName
  (params (PlayerState :type BP%20Truck%20Player%20State%20Object%20Reference) (CharacterName :type String))
  (Variables|BP_TruckPlayerState_C|SetCharacterName PlayerState CharacterName))

(fn ConstructionScript)

(fn BPTruckPlayerStateAutoGenFunc
  (Variables|Default|SetLastScoreIncrease 0))