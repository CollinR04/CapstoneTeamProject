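; BP_SuspensionWheel is a wheel visual for the custom player truck that follows its suspension travel.
; Each tick it sets its relative Z by interpolating from the suspension's max extension to zero using the current compression amount.
; Two replicated material variables apply themselves to mesh slots 0 and 1 through their OnRep functions, syncing the wheel's look across clients.
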(event EventTick
  (params (DeltaSeconds :type Float%20%28single-precision%29))
  (bind _suspension (Variables|Default|GetSuspension))
  (Transformation|SetRelativeLocation (Math|Vector|MakeVector 0.0 0.0 (Math|Float|Lerp (Variables|/Script/ChaosTruck.TruckSuspension|GetMaxExtension _suspension) 0.0 (Variables|/Script/ChaosTruck.TruckSuspension|GetCompressionAmount _suspension))) false false))

(fn OnRepMat0
  (Rendering|Material|SetMaterial 0 (Variables|Default|GetMat0)))

(fn OnRepMat1
  (Rendering|Material|SetMaterial 1 (Variables|Default|GetMat1)))