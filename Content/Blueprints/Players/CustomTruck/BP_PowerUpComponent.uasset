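; BP_PowerUpComponent handles power-up pickup for BP_Truck players.
; PowerUpCollision casts the truck, its player controller and the BP_Pickup, and if the inventory's GetPickUp check passes, stores the item in PlayerInventory and copies its name to the controller's RepName.
; BP_CheckForItems repeats this after the current power-up expires, but passes "None" as the inventory item name.
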(event Custom|PowerUpCollision
  (params (TruckActor :type Actor%20Object%20Reference) (PowerUpActor :type Actor%20Object%20Reference))
  ;[0.15 0.15 0.15 0.5] Power-up pickup
  (bind _asbp_truck (Utilities|Casting|CastToBP_Truck TruckActor))
  (bind _asbp_truck_player_controller (Utilities|Casting|CastToBP_TruckPlayerController (Pawn|GetController _asbp_truck)))
  (bind _asbp_pickup (Utilities|Casting|CastToBP_Pickup PowerUpActor))
  (bind _returnvalue (Class|PlayerInventory|GetPickUp (Variables|/Game/Blueprints/Players/CustomTruck/BP_Truck.BP_Truck_C|GetPlayerInventory _asbp_truck)))
  (if _returnvalue
    (Class|PlayerInventory|PickUpItem (Variables|/Game/Blueprints/Players/CustomTruck/BP_Truck.BP_Truck_C|GetPlayerInventory _asbp_truck) (Variables|/Script/ChaosTruck.PowerUp|GetPowerUpNum _asbp_pickup) (Variables|/Script/ChaosTruck.PowerUp|GetPowerUpName _asbp_pickup))
    (Variables|/Game/Blueprints/Players/CustomTruck/BP_TruckPlayerController.BP_TruckPlayerController_C|SetRepName _asbp_truck_player_controller (Variables|/Script/ChaosTruck.PowerUp|GetPowerUpName _asbp_pickup))))

(event Custom|BP_CheckForItems
  (params (TruckActor :type Actor%20Object%20Reference) (OtherActor :type Actor%20Object%20Reference))
  ;[0.15 0.15 0.15 0.5] Check for power-ups after current power-up expires
  (bind _asbp_truck (Utilities|Casting|CastToBP_Truck TruckActor))
  (bind _asbp_truck_player_controller (Utilities|Casting|CastToBP_TruckPlayerController (Pawn|GetController _asbp_truck)))
  (bind _asbp_pickup (Utilities|Casting|CastToBP_Pickup OtherActor))
  (bind _returnvalue (Class|PlayerInventory|GetPickUp (Variables|/Game/Blueprints/Players/CustomTruck/BP_Truck.BP_Truck_C|GetPlayerInventory _asbp_truck)))
  (if _returnvalue
    (Class|PlayerInventory|PickUpItem (Variables|/Game/Blueprints/Players/CustomTruck/BP_Truck.BP_Truck_C|GetPlayerInventory _asbp_truck) (Variables|/Script/ChaosTruck.PowerUp|GetPowerUpNum _asbp_pickup) "None")
    (Variables|/Game/Blueprints/Players/CustomTruck/BP_TruckPlayerController.BP_TruckPlayerController_C|SetRepName _asbp_truck_player_controller (Variables|/Script/ChaosTruck.PowerUp|GetPowerUpName _asbp_pickup))))

(event EventBeginPlay)

(event EventTick
  (params (DeltaSeconds :type Float%20%28single-precision%29)))