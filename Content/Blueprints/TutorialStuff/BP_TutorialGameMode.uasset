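; Tutorial game mode, derived from BP_TestGameMode, that sequences truck tutorial challenges and narrative.
; Objective markers from the construction script trigger challenges by number; damage and power-up events are empty stubs.
; The breakable challenge spawns random breakables near the second marker and counts their destruction through the challenge widget.
; Marker hits and challenge completion show narrative and swap truck input for menu input until the narrative completes.
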(event Custom|MarkerReached
  (params (Narrative%20Number :type Integer) (ChallengeNumber :type Integer))
  (Variables|NarrativeStuff|SetNarrativeNum Narrative%20Number)
  (if (!= ChallengeNumber -1)
    (bind _output_get (Variables|ChallengeStuff|SetChallengeNum ChallengeNumber))
    (switch int _output_get
      (:0
        (CallFunction|StartDriveEvent))
      (:1
        (CallFunction|StartBreakableEvent))
      (:2
        (CallFunction|StartDamageEvent))
      (:3
        (CallFunction|StartPowerUpEvent)))))

(event EventBeginPlay
  (bind _levelmarkers (Variables|Default|GetLevelMarkers))
  (|CallParentFunction) ; Parent is BP_TestGameMode
  (CallFunction|SetUpWidgets)
  (CallFunction|LinkTutorialDelagates)
  (EventDispatchers|BindEventtoOnMarkerReached _levelmarkers (delegate Custom|MarkerReached))
  (Variables|BreakableStuff|SetBreakableLocation (Transformation|GetActorLocation (Utilities|Array|Get(acopy) _levelmarkers 1))))

(event EventTick
  (params (DeltaSeconds :type Float%20%28single-precision%29))
  (|CallParentFunction DeltaSeconds) ; Parent is BP_TestGameMode
)

(event Custom|StartBreakableEvent
  ;[0.15 0.15 0.15 0.5] Normal breakable event
  (BreakableStuff|SpawnBreakables)
  (Utilities|FlowControl|Delay 0.2)
  (bind _outactors (Actor|GetAllActorsOfClass "/Game/Blueprints/TutorialStuff/BP_TutorialBreakable.BP_TutorialBreakable_C"))
  (Variables|Default|SetAll%20Breakables _outactors)
  (EventDispatchers|BindEventtoOnTutorialDestroyed _outactors (delegate Custom|ObjectDestroyed))
  (BreakableStuff|UpdateBreakableUI))

(event Custom|ObjectDestroyed
  ;[0.15 0.15 0.15 0.5] Normal breakable event
  (Math|Integer|IncrementInt (Variables|BreakableStuff|GetBreakableCount)
    (:%20%20
      (BreakableStuff|UpdateBreakableUI))))

(event Custom|EndBreakableEvent
  ;[0.15 0.15 0.15 0.5] End of breakable event
  (Variables|NarrativeStuff|SetNarrativeNum (Variables|ChallengeStuff|GetPostBreakableNarrativeNum))
  (Development|PrintString (Utilities|String|ToString(Integer) (Variables|BreakableStuff|GetBreakableCount)))
  (Default|CallChallengeCompleted (Variables|UIWidget|GetChallengeWidget)))

(event Custom|ReverseBreakableEvent)

(event Custom|StartDamageEvent)

(event Custom|StartPowerUpEvent)

(event Custom|StartDriveEvent
  (Default|SetObjective (Variables|UIWidget|GetChallengeWidget) (Variables|ChallengeStuff|GetChallengeNum) false))

(event Custom|PauseGame2
  (bind _narrativewidget (Variables|UIWidget|GetNarrativeWidget))
  (bind _asbp_truck_player_controller (Utilities|Casting|CastToBP_TruckPlayerController (Game|GetPlayerController 0)))
  (Input|RemoveMappingContext (PlayerController|LocalPlayerSubsystems|GetEnhancedInputLocalPlayerSubsystem _asbp_truck_player_controller) "/Game/Input/IMC_TruckInputs.IMC_TruckInputs" "(bIgnoreAllPressedKeysUntilRelease=True,bForceImmediately=False,bNotifyUserSettings=False)")
  (Input|AddMappingContext (PlayerController|LocalPlayerSubsystems|GetEnhancedInputLocalPlayerSubsystem _asbp_truck_player_controller) "/Game/Input/IMC_MenuInputs.IMC_MenuInputs" 0 "(bIgnoreAllPressedKeysUntilRelease=True,bForceImmediately=False,bNotifyUserSettings=False)")
  (Default|SetNextNarrative _narrativewidget)
  (Widget|SetVisibility _narrativewidget "Visible"))

(event Custom|UnpauseGame
  (bind _asbp_truck_player_controller (Utilities|Casting|CastToBP_TruckPlayerController (Game|GetPlayerController 0)))
  (Input|RemoveMappingContext (PlayerController|LocalPlayerSubsystems|GetEnhancedInputLocalPlayerSubsystem _asbp_truck_player_controller) "/Game/Input/IMC_MenuInputs.IMC_MenuInputs" "(bIgnoreAllPressedKeysUntilRelease=True,bForceImmediately=False,bNotifyUserSettings=False)")
  (Input|AddMappingContext (PlayerController|LocalPlayerSubsystems|GetEnhancedInputLocalPlayerSubsystem _asbp_truck_player_controller) "/Game/Input/IMC_TruckInputs.IMC_TruckInputs" 0 "(bIgnoreAllPressedKeysUntilRelease=True,bForceImmediately=False,bNotifyUserSettings=False)")
  (Widget|SetVisibility (Variables|UIWidget|GetNarrativeWidget) "Hidden"))

(event Custom|PauseGame
  (params (Narrative%20Number :type Integer) (ChallengeNumber :type Integer))
  (bind _narrativewidget (Variables|UIWidget|GetNarrativeWidget))
  (bind _asbp_truck_player_controller (Utilities|Casting|CastToBP_TruckPlayerController (Game|GetPlayerController 0)))
  (Input|RemoveMappingContext (PlayerController|LocalPlayerSubsystems|GetEnhancedInputLocalPlayerSubsystem _asbp_truck_player_controller) "/Game/Input/IMC_TruckInputs.IMC_TruckInputs" "(bIgnoreAllPressedKeysUntilRelease=True,bForceImmediately=False,bNotifyUserSettings=False)")
  (Input|AddMappingContext (PlayerController|LocalPlayerSubsystems|GetEnhancedInputLocalPlayerSubsystem _asbp_truck_player_controller) "/Game/Input/IMC_MenuInputs.IMC_MenuInputs" 0 "(bIgnoreAllPressedKeysUntilRelease=True,bForceImmediately=False,bNotifyUserSettings=False)")
  (Default|SetNextNarrative _narrativewidget)
  (Widget|SetVisibility _narrativewidget "Visible"))

(event Custom|LinkTutorialDelagates
  (Utilities|FlowControl|Delay 0.2)
  (Input|SetInputModeGameandUI (Game|GetPlayerController 0) (Variables|UIWidget|GetScoreWidget) "DoNotLock" true false)
  (bind _asbp_tutorial_game_mode (Utilities|Casting|CastToBP_TutorialGameMode (Game|GetGameMode)))
  (EventDispatchers|BindEventtoOnMarkerReached (Variables|BP_TutorialGameMode_C|GetLevelMarkers _asbp_tutorial_game_mode) (delegate Custom|PauseGame))
  (EventDispatchers|BindEventtoChallengeCompleted (Variables|UIWidget|GetChallengeWidget) (delegate Custom|PauseGame2))
  (EventDispatchers|BindEventtoCompletedNarrative (Variables|UIWidget|GetNarrativeWidget) (delegate Custom|UnpauseGame)))

(fn ConstructionScript
  (|CallParentFunction)
  (bind _outactors (Actor|GetAllActorsOfClass "/Game/Blueprints/TutorialStuff/BP_TutorialObjectiveMarker.BP_TutorialObjectiveMarker_C"))
  (Variables|Default|SetLevelMarkers _outactors))

(fn SpawnBreakables
  (bind _breakablelocation (Variables|BreakableStuff|GetBreakableLocation))
  (bind _breakable_types (Variables|BreakableStuff|GetBreakable%20Types))
  (bind (_x _y) (Math|Vector|BreakVector _breakablelocation))
  (while (!= (Variables|BreakableStuff|GetBreakableCount) (Variables|BreakableStuff|GetBreakableTotal))
    (Math|Integer|IncrementInt (Variables|BreakableStuff|GetBreakableCount)
      (:%20%20
        (Game|SpawnActorfromClass (Utilities|Array|Get(acopy) _breakable_types (Math|Random|RandomIntegerinRange 0 (- (Utilities|Array|Length _breakable_types) 1))) (Math|Transform|MakeTransform (Math|Vector|MakeVector (Math|Random|RandomFloatinRange (+ _x (Variables|BreakableStuff|GetMin%20Spawn%20Range%20Add)) (+ _x (Variables|BreakableStuff|GetMax%20Spawn%20Range%20Add))) (Math|Random|RandomFloatinRange (+ _y (Variables|BreakableStuff|GetMin%20Spawn%20Range%20Add)) (+ _y (Variables|BreakableStuff|GetMax%20Spawn%20Range%20Add))) 0.0)) "Undefined" "MultiplyWithRoot" 0 0))))
  (Variables|BreakableStuff|SetBreakableCount 0))

(fn UpdateBreakableUI
  (Default|SetObjective (Variables|UIWidget|GetChallengeWidget) (Variables|ChallengeStuff|GetChallengeNum) true (Variables|BreakableStuff|GetBreakableCount) (Variables|BreakableStuff|GetBreakableTotal))
  (if (== (Variables|BreakableStuff|GetBreakableCount) (Variables|BreakableStuff|GetBreakableTotal))
    (Default|CompleteObjective (Variables|UIWidget|GetChallengeWidget))
    (CallFunction|EndBreakableEvent)))

(fn SetUpWidgets
  (bind _returnvalue (Game|GetPlayerController 0))
  (bind _returnvalue_2 (UserInterface|CreateWidget "/Game/Blueprints/UI/Tutorial/WBP_TutorialNarrative.WBP_TutorialNarrative_C" _returnvalue))
  (bind _output_get (Variables|UIWidget|SetNarrativeWidget _returnvalue_2))
  (bind _returnvalue_3 (UserInterface|CreateWidget "/Game/Blueprints/UI/Tutorial/WBP_TutorialChallenge.WBP_TutorialChallenge_C" _returnvalue))
  (bind _output_get_2 (Variables|UIWidget|SetChallengeWidget _returnvalue_3))
  (bind _returnvalue_4 (UserInterface|CreateWidget "/Game/Blueprints/UI/InGameHUD/BP_ScoreHUD.BP_ScoreHUD_C" _returnvalue))
  (bind _output_get_3 (Variables|UIWidget|SetScoreWidget _returnvalue_4))
  (UserInterface|Viewport|AddtoViewport _output_get 0)
  (Widget|SetVisibility (Variables|UIWidget|GetNarrativeWidget) "Hidden"))