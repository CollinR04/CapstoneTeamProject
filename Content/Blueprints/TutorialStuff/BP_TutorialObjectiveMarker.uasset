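; BP_TutorialObjectiveMarker is a tutorial objective marker that reports when its trigger box is reached.
; The construction script sizes the box to TriggerSize, or destroys it when UseTrigger is off.
; Any overlap while Enabled clears the flag through EnableObjectiveMarker, then calls OnMarkerReached with the marker's NarrativeNumber and ChallengeNumber.
; EnableObjectiveMarker only stores its two flags, and DisableOnReached is never checked here.
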(event OnComponentBeginOverlap(CollsionBox)
  (params (OverlappedComponent :type Primitive%20Component%20Object%20Reference) (OtherActor :type Actor%20Object%20Reference) (OtherComp :type Primitive%20Component%20Object%20Reference) (OtherBodyIndex :type Integer) (bFromSweep :type Boolean) (SweepResult :type Hit%20Result%20Structure%20%28by%20ref%29))
  (if (Variables|ObjectiveMarker|GetEnabled)
    (CallFunction|EnableObjectiveMarker false true) ; Disable this objective
    (Default|CallOnMarkerReached (Variables|ObjectiveMarker|GetNarrativeNumber) (Variables|ObjectiveMarker|GetChallengeNumber))))

(fn ConstructionScript
  (bind _collsionbox (Variables|Default|GetCollsionBox))
  (if (Variables|ObjectiveMarker|GetUseTrigger)
    (Components|Box|SetBoxExtent _collsionbox (Variables|ObjectiveMarker|GetTrigger%20Size) true)
    (else
      (Components|DestroyComponent _collsionbox))))

(fn EnableObjectiveMarker
  (params (Enable :type Boolean) (DisableOnReached :type Boolean))
  (Variables|ObjectiveMarker|SetEnabled Enable)
  (Variables|ObjectiveMarker|SetDisableOnReached DisableOnReached))