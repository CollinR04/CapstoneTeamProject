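; Team deathmatch game mode for truck players that splits them into two teams and colors their spotlights by team.
; On BeginPlay it sets the game state's mode, then the server polls until exactly four pawns exist.
; The first two player states become team one, the rest team two.
; After a kill and respawn it reapplies the player's spotlight color; the scoring event is only a stub.
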(event Custom|TDM_Scoring
  (bind _asgs_gtdagame_state (Utilities|Casting|CastToGS_GTDAGameState (Game|GetGameState))))

(event Custom|AssignTeams
  (params (TeamOne :type Array%20of%20Integers))
  ;[0.15 0.15 0.15 0.5] Assign Teams
  (for _index (range 0 (- (Class|GameplayStatics|GetNumPlayerStates) 1))
    (if (Utilities|Array|ContainsItem TeamOne _index)
      (bind _asbp_truck_player_state (Utilities|Casting|CastToBP_TruckPlayerState (Game|GetPlayerState _index)))
      (Variables|/Script/ChaosTruck.TruckPlayerState|SetTeamID _asbp_truck_player_state 1)
      (else
        (bind _asbp_truck_player_state_2 (Utilities|Casting|CastToBP_TruckPlayerState (Game|GetPlayerState _index)))
        (Variables|/Script/ChaosTruck.TruckPlayerState|SetTeamID _asbp_truck_player_state_2 2)))
    (Default|ChangeSpotlightColorState _asbp_truck_player_state_2)))

(event EventBeginPlay
  ;[0.15 0.15 0.15 0.5] Wait for players and assign teams
  (|CallParentFunction)
  (bind _asgs_gtdagame_state (Utilities|Casting|CastToGS_GTDAGameState (Game|GetGameState)))
  (Variables|/Game/Blueprints/Backend/GS_GTDAGameState.GS_GTDAGameState_C|SetGameMode _asgs_gtdagame_state "NewEnumerator2")
  (Networking|SwitchHasAuthority
    (:Authority
      (bind _outactors (Actor|GetAllActorsOfClass "/Script/Engine.Pawn" :!label _label))
      (if (== (Utilities|Array|Length _outactors) 4)
        (CallFunction|AssignTeams (Utilities|Array|MakeArray 0 1))
        (else
          (Utilities|FlowControl|Delay 0.2)
          (goto _label))))))

(event EventOnKillandRespawn
  (params (Controller :type Controller%20Object%20Reference))
  (|CallParentFunction Controller)
  (bind _asbp_truck_player_state (Utilities|Casting|CastToBP_TruckPlayerState (Variables|/Script/Engine.Controller|GetPlayerState Controller)))
  (Default|ChangeSpotLightColorReplicated _asbp_truck_player_state))

(fn ConstructionScript)