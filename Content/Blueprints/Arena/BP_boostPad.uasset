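; BP_boostPad is an arena boost pad Actor that detects overlapping BP_Truck actors, but currently applies no boost.
; On BeginPlay it activates its InterpToMovement component.
; Box and actor overlaps share a class check and cast to BP_Truck, where the chain ends.
; Unconnected leftover nodes would push the truck chassis along its velocity or launch a character upward.
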(event OnComponentBeginOverlap(Box)
  (params (OverlappedComponent :type Primitive%20Component%20Object%20Reference) (OtherActor :type Actor%20Object%20Reference) (OtherComp :type Primitive%20Component%20Object%20Reference) (OtherBodyIndex :type Integer) (bFromSweep :type Boolean) (SweepResult :type Hit%20Result%20Structure%20%28by%20ref%29))
  (Class|KismetSystemLibrary|IsObjectOfSoftClass OtherActor "/Game/Blueprints/Players/CustomTruck/BP_Truck.BP_Truck_C"
    (:True
      (bind _asbp_truck (Utilities|Casting|CastToBP_Truck OtherActor)))))

(event EventBeginPlay
  (Components|Activation|Activate (Variables|Default|GetInterpToMovement) false))

(event Collision|EventActorBeginOverlap
  (params (OtherActor :type Actor%20Object%20Reference))
  (Class|KismetSystemLibrary|IsObjectOfSoftClass (stale OnComponentBeginOverlap(Box) OtherActor) "/Game/Blueprints/Players/CustomTruck/BP_Truck.BP_Truck_C"
    (:True
      (bind _asbp_truck (Utilities|Casting|CastToBP_Truck (stale OnComponentBeginOverlap(Box) OtherActor))))))

(event EventTick
  (params (DeltaSeconds :type Float%20%28single-precision%29)))

(fn ConstructionScript)