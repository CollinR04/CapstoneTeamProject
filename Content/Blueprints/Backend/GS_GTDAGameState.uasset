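; Game state that coordinates pre-match map and character selection, player readiness and map travel.
; Ready functions swap menu and truck input contexts; when the ready count matches NumPlayers, it shows a loading screen, then travels through the game instance after a delay.
; Map-selection widgets are updated directly, with text changes limited to clients.
; RepNotifies propagate locked-character and map changes and play death explosion effects and sound.
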(event Custom|ShowLoadingScreeb
  (bind _returnvalue (UserInterface|CreateWidget "/Game/Blueprints/UI/LoadingScreen.LoadingScreen_C" (Game|GetPlayerController 0)))
  (UserInterface|Viewport|AddtoViewport _returnvalue 0))

(event Custom|RemovePlayer
  (bind _result (Math|Integer|DecrementInt (Variables|Default|GetNumPlayersReady))
    (:%20%20
      (Variables|Default|SetNumPlayersReady _result))))

(event Custom|UpdateUI
  (Networking|SwitchHasAuthority
    (:Remote
      (bind _foundwidgets (Widget|GetAllWidgetsOfClass "/Game/Blueprints/UI/BP_MapSelcetion.BP_MapSelcetion_C" true))
      (for _array_element _foundwidgets
        (Variables|/Script/UMG.TextBlock|SetText (Variables|/Game/Blueprints/UI/BP_MapSelcetion.BP_MapSelcetion_C|Gettext_SelectedMap _array_element) (Variables|Default|GetSelectedMapName))
        (Variables|/Script/UMG.TextBlock|SetText (Variables|/Game/Blueprints/UI/BP_MapSelcetion.BP_MapSelcetion_C|Gettext_desc _array_element) (Variables|Default|Getmap_desctext))))))

(event Custom|UpdateGameImage
  (bind _foundwidgets (Widget|GetAllWidgetsOfClass "/Game/Blueprints/UI/BP_MapSelcetion.BP_MapSelcetion_C" true))
  (for _array_element _foundwidgets
    (bind _astexture_2d (Utilities|Casting|CastToTexture2D (.ResourceObject (Utilities|Struct|BreakSlateBrush (Variables|/Script/UMG.Image|GetBrush (Variables|/Game/Blueprints/UI/BP_MapSelcetion.BP_MapSelcetion_C|GetGamemode_Icon _array_element))))))
    (if (== _astexture_2d "/Game/UIAssets/MAP_SELECT/MAP_SELECT_NEWICONS/Map-select_TEAMDEATHMATCH_ICON_2_0.Map-select_TEAMDEATHMATCH_ICON_2_0")
      (Appearance|SetBrushfromTexture (Variables|/Game/Blueprints/UI/BP_MapSelcetion.BP_MapSelcetion_C|GetGamemode_Icon _array_element) "/Game/UIAssets/MAP_SELECT/MAP_SELECT_NEWICONS/Map-select_FREEFORALL_ICON_2_0.Map-select_FREEFORALL_ICON_2_0" false)
      (else
        (Appearance|SetBrushfromTexture (Variables|/Game/Blueprints/UI/BP_MapSelcetion.BP_MapSelcetion_C|GetGamemode_Icon _array_element) "/Game/UIAssets/MAP_SELECT/MAP_SELECT_NEWICONS/Map-select_TEAMDEATHMATCH_ICON_2_0.Map-select_TEAMDEATHMATCH_ICON_2_0" false)))))

(event Custom|Update%20Text
  (params (Text%20Mode :type Text))
  (Networking|SwitchHasAuthority
    (:Remote
      (bind _foundwidgets (Widget|GetAllWidgetsOfClass "/Game/Blueprints/UI/BP_MapSelcetion.BP_MapSelcetion_C" true))
      (for _array_element _foundwidgets
        (Variables|/Script/UMG.TextBlock|SetText (Variables|/Game/Blueprints/UI/BP_MapSelcetion.BP_MapSelcetion_C|GetText_Mode _array_element) Text%20Mode)))))

(event Custom|AddPlayer
  (bind _numplayers (Variables|Default|GetNumPlayers))
  (bind _numplayersready (Variables|Default|GetNumPlayersReady))
  (bind _result (Math|Integer|IncrementInt _numplayersready)
    (:%20%20
      (Development|PrintString (Utilities|String|Append "Player State Num:" (Utilities|String|ToString(Integer) _numplayers)))
      (Development|PrintString (Utilities|String|Append "Players Ready: " (Utilities|String|ToString(Integer) _numplayersready)))
      (if (== _numplayers _result)
        (CallFunction|ShowLoadingScreeb)
        (Utilities|FlowControl|Delay 5.0)
        (CallFunction|StartGame)
        (else
          (Development|PrintString "Number not met"))))))

(event EventBeginPlay
  (Variables|Default|SetNumPlayers (Class|GameplayStatics|GetNumPlayerControllers)))

(event Custom|LockCharacter%28Server%29
  (params (Character%20Name :type String))
  (Utilities|Array|AddUnique (Variables|Default|GetLockedCharacters) Character%20Name))

(fn ConstructionScript)

(fn StartGame
  (CallFunction|ChangeMap (Variables|Default|GetStartGameMap)))

(fn PlayerReady
  (params (PlayerController :type Player%20Controller%20Object%20Reference))
  (bind _asbp_truck_player_controller (Utilities|Casting|CastToBP_TruckPlayerController PlayerController))
  (Input|RemoveMappingContext (PlayerController|LocalPlayerSubsystems|GetEnhancedInputLocalPlayerSubsystem _asbp_truck_player_controller) "/Game/Input/IMC_MenuInputs.IMC_MenuInputs" "(bIgnoreAllPressedKeysUntilRelease=True,bForceImmediately=False,bNotifyUserSettings=False)")
  (Input|AddMappingContext (PlayerController|LocalPlayerSubsystems|GetEnhancedInputLocalPlayerSubsystem _asbp_truck_player_controller) "/Game/Input/IMC_TruckInputs.IMC_TruckInputs" 0 "(bIgnoreAllPressedKeysUntilRelease=True,bForceImmediately=False,bNotifyUserSettings=False)")
  (Default|ReadyUpPlayeronServer _asbp_truck_player_controller))

(fn ChangeMap
  (params (MapName :type String))
  ;[0.15 0.15 0.15 0.5] Change Map Command
  (bind _asbp_test_game_mode (Utilities|Casting|CastToBP_TestGameMode (Game|GetGameMode)))
  (bind _asbp_truck_game_instance (Utilities|Casting|CastToBP_TruckGameInstance (Game|GetGameInstance)))
  (Default|TraveltoMap _asbp_truck_game_instance MapName (Variables|Default|GetNumPlayers) (Variables|/Game/Blueprints/BP_TestGameMode.BP_TestGameMode_C|GetCurrentGameMode _asbp_test_game_mode)))

(fn OnRepNumPlayersReady)

(fn OnRepLockedCharacters
  (Default|CallCharacterSelectUpdate)
  (Development|PrintString "Hello"))

(fn LockCharcter
  (params (CharacterName :type String))
  (Utilities|Array|AddUnique (Variables|Default|GetLockedCharacters) CharacterName)
  (Variables|Default|SetLockedCharacters (Variables|Default|GetLockedCharacters)))

(fn UnlockCharacter
  (params (CharacterName :type String))
  (Utilities|Array|RemoveItem (Variables|Default|GetLockedCharacters) CharacterName))

(fn PlayerUnReady
  (params (PlayerController :type Player%20Controller%20Object%20Reference))
  (bind _asbp_truck_player_controller (Utilities|Casting|CastToBP_TruckPlayerController PlayerController))
  (Input|RemoveMappingContext (PlayerController|LocalPlayerSubsystems|GetEnhancedInputLocalPlayerSubsystem _asbp_truck_player_controller) "/Game/Input/IMC_TruckInputs.IMC_TruckInputs" "(bIgnoreAllPressedKeysUntilRelease=True,bForceImmediately=False,bNotifyUserSettings=False)")
  (Input|AddMappingContext (PlayerController|LocalPlayerSubsystems|GetEnhancedInputLocalPlayerSubsystem _asbp_truck_player_controller) "/Game/Input/IMC_MenuInputs.IMC_MenuInputs" 0 "(bIgnoreAllPressedKeysUntilRelease=True,bForceImmediately=False,bNotifyUserSettings=False)")
  (Default|UnReadyUpPlayeronServer _asbp_truck_player_controller))

(fn OnRepDeadPlayerLocation
  (bind _deadplayerlocation (Variables|Default|GetDeadPlayerLocation))
  (Niagara|SpawnSystematLocation "/Game/VFX/ParticleSystems/PS_Death_Explosion.PS_Death_Explosion" _deadplayerlocation "0, 0, 0" "2.000000,2.000000,2.000000")
  (Audio|PlaySoundatLocation "/Game/Audio/SFX/gtda_deathexplosion_v2.gtda_deathexplosion_v2" _deadplayerlocation "0, 0, 0" 1.0 1.0 0.0 0 0 0 0))

(fn OnRepMapName
  (Default|CallOnMapSelect))