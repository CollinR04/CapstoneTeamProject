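; Truck game instance that handles server map travel by game mode and toggles the local pause menu.
; TravelToMap stamps the mode on cached controllers' player states, server-travels via a SetGameMode-built URL, then, under BP_TestGameMode, refreshes that controller cache and sets the GameState's mode.
; Togglepause flips the pause flags, creating and reusing one menu widget and switching player 0's input mode and cursor, without pausing the world itself.
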(event Custom|TravelToMap
  (params (Map%20Name :type String) (Num_Players :type Integer) (CurrntGamemode :type E_GameMode%20Enum :default "NewEnumerator1"))
  (bind _returnvalue (Game|GetGameMode))
  ;[0.15 0.15 0.15 0.5] Map Travel
  (for _array_element (Variables|Default|GetPlayerControllers)
    (bind _asbp_truck_player_state (Utilities|Casting|CastToBP_TruckPlayerState (Variables|/Script/Engine.Controller|GetPlayerState _array_element)))
    (Variables|/Game/Blueprints/Players/CustomTruck/BP_TruckPlayerState.BP_TruckPlayerState_C|SetActiveGameMode _asbp_truck_player_state CurrntGamemode))
  (Variables|Default|SetNum_Players Num_Players)
  (bind _returnvalue_2 (Class|GTDAGameInstance|SetGameMode (Utilities|String|EnumtoString CurrntGamemode) Map%20Name))
  (Class|AdvancedSessionsLibrary|ServerTravel _returnvalue_2 false false)
  (if (Class|GameplayStatics|ObjectIsA _returnvalue "/Game/Blueprints/BP_TestGameMode.BP_TestGameMode_C")
    (bind _asbp_test_game_mode (Utilities|Casting|CastToBP_TestGameMode _returnvalue))
    (Variables|Default|SetPlayerControllers (Variables|/Game/Blueprints/BP_TestGameMode.BP_TestGameMode_C|GetAll_ConnectedControllers _asbp_test_game_mode))
    (Development|PrintString (Utilities|String|ToString(Integer) (Utilities|Array|Length (Variables|/Game/Blueprints/BP_TestGameMode.BP_TestGameMode_C|GetAll_ConnectedControllers _asbp_test_game_mode))))
    (bind _asgs_gtdagame_state (Utilities|Casting|CastToGS_GTDAGameState (Game|GetGameState)))
    (bind _output_get (Variables|/Game/Blueprints/Backend/GS_GTDAGameState.GS_GTDAGameState_C|SetGameMode _asgs_gtdagame_state CurrntGamemode))
    (Development|PrintString (Utilities|String|EnumtoString _output_get) true true "(R=1.000000,G=0.148157,B=0.068792,A=1.000000)" 15.0)))

(fn UIShowPauseMenu
  (bind _returnvalue (Game|GetPlayerController 0))
  (Utilities|IsValid (Variables|Default|GetWb_PauseMenu)
    (:Is%20Valid
      _)
    (:Is%20Not%20Valid
      (bind _returnvalue_2 (UserInterface|CreateWidget "/Game/Blueprints/UI/BP_PauseMenu.BP_PauseMenu_C" _returnvalue))
      (Variables|Default|SetWb_PauseMenu _returnvalue_2)))
  (UserInterface|Viewport|AddtoViewport (Variables|Default|GetWb_PauseMenu) 0)
  (Input|SetInputModeUIOnly _returnvalue (Variables|/Game/Blueprints/UI/BP_PauseMenu.BP_PauseMenu_C|GetResumeGame_Button _returnvalue_2) "DoNotLock" false)
  (Variables|/Script/Engine.PlayerController|SetbShowMouseCursor _returnvalue true)
  (return))

(fn Togglepause
  (bind _returnvalue (Game|GetPlayerController 0))
  (if (Variables|Default|GetPauseMenuVis)
    (Variables|Default|SetPauseMenuVis false)
    (Variables|Default|SetIsGamePause false)
    (Widget|RemovefromParent (Variables|Default|GetWb_PauseMenu))
    (Input|SetInputModeGameOnly _returnvalue false)
    (Variables|/Script/Engine.PlayerController|SetbShowMouseCursor _returnvalue false)
    (bind _asbp_truck_controller (Utilities|Casting|CastToBP_TruckController _returnvalue))
    (Default|UnhidePauseMenu _asbp_truck_controller)
    (else
      (Variables|Default|SetPauseMenuVis true)
      (Variables|Default|SetIsGamePause true)
      (CallFunction|UIShowPauseMenu)))
  (return (Variables|Default|GetIsGamePause)))