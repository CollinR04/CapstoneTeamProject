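; BP_Shell is a truck's armor shell, grouping BP_ArmorCollection components and handling their damage, break and shield effects.
; On BeginPlay it binds to each collection and re-broadcasts truck damage, collection-empty and armor-broken events through its own dispatchers.
; Armor breaks spawn a particle system using the broken piece's mesh, and shield particles toggle, both replicated via server-to-multicast RPCs.
; SetSpeedThreshold passes a speed threshold to every collection.
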(event EventBeginPlay
  (bind _returnvalue (Actor|GetComponentsByClass "/Game/Blueprints/Armor/BP_ArmorCollection.BP_ArmorCollection_C"))
  ;[0.15 0.15 0.15 0.5] Bind collections to event
  (Variables|Default|SetArmorCollections _returnvalue)
  (for _array_element _returnvalue
    (EventDispatchers|BindEventtoOnTruckDamage _array_element (EventDispatchers|CreateEvent :!event Custom|BroadcastTruckDamage))
    ;[0.15 0.15 0.15 0.5] Bind for powerup damage logic
    (EventDispatchers|BindEventtoOnCollectionEmpty _array_element (EventDispatchers|CreateEvent :!event Custom|CheckCollectionsEmpty))
    (EventDispatchers|BindEventtoOnArmorBroken _array_element (EventDispatchers|CreateEvent :!event Custom|ArmorBreakEvent))))

(event Custom|BroadcastTruckDamage
  (params (Damage :type Float%20%28double-precision%29) (OtherActor :type Actor%20Object%20Reference))
  ;[0.15 0.15 0.15 0.5] Broadcast so truck can take damage
  (Default|CallOnTruckDamageNotify Damage OtherActor))

(event Custom|CheckCollectionsEmpty
  (params (bIsEmpty :type Boolean))
  (Default|CallOnCollectionEmptyNotify bIsEmpty))

(event Custom|ArmorBreakEvent
  (params (BrokenArmor :type Armor%20Object%20Reference))
  (Default|CallOnArmorBreakNotify BrokenArmor)
  (CallFunction|CreateParticles BrokenArmor))

(event Custom|Server_CreateParticles
  (params (BrokenArmor :type Static%20Mesh%20Component%20Object%20Reference))
  (CallFunction|MulticastCreateParticles BrokenArmor))

(event Custom|Multicast_CreateParticles
  (params (BrokenMesh :type Static%20Mesh%20Component%20Object%20Reference))
  (bind _returnvalue (Niagara|SpawnSystemAttached "/Game/VFX/ParticleSystems/PS_ArmorBreak.PS_ArmorBreak" BrokenMesh "None" "0, 0, 0" "0, 0, 0" "KeepRelativeOffset" true))
  (Class|NiagaraComponent|SetVariableStaticMesh _returnvalue "BrokenMesh" (Variables|/Script/Engine.StaticMeshComponent|GetStaticMesh BrokenMesh)))

(event Custom|CreateParticles
  (params (Broken%20Armor :type Static%20Mesh%20Component%20Object%20Reference))
  (Networking|SwitchHasAuthority
    (:Authority
      (CallFunction|MulticastCreateParticles Broken%20Armor))
    (:Remote
      (CallFunction|ServerCreateParticles Broken%20Armor))))

(event Custom|Multicast_ActivateShield
  (params (bIsActive :type Boolean))
  (bind _shieldparticles (Variables|Default|GetShieldParticles))
  (Utilities|IsValid _shieldparticles
    (:Is%20Valid
      (Components|Activation|SetActive _shieldparticles bIsActive false))))

(event Custom|ActivateShield
  (params (bIsActive :type Boolean))
  (if (Ability|HasAuthority (Components|GetOwner))
    (CallFunction|MulticastActivateShield bIsActive)
    (else
      (CallFunction|ServerActivateShield bIsActive))))

(event Custom|Server_ActivateShield
  (params (bIsActive :type Boolean))
  (CallFunction|MulticastActivateShield bIsActive))

(fn ConstructionScript)

(fn SetSpeedThreshold
  (params (SpeedThreshold :type Float%20%28double-precision%29))
  (for _array_element (Actor|GetComponentsByClass "/Game/Blueprints/Armor/BP_ArmorCollection.BP_ArmorCollection_C")
    (Variables|/Script/ChaosTruck.ArmorCollection|SetSpeedThreshold _array_element SpeedThreshold)))

(fn OnRepCurrentVel)