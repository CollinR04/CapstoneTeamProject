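; BP_YellowShell is an armor shell Blueprint, set apart by a NonDestructables component that GetRoot returns as its root.
; Its construction script does no work.
; Unwired loops in that script would reparent BP_ArmorCollection and BP_Armor components to NonDestructables, keeping world transforms, but they never run.
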(fn ConstructionScript)

(fn GetRoot
  (return (Variables|Default|GetNonDestructables)))