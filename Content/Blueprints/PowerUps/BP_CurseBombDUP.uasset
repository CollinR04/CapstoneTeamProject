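; Curse bomb power-up actor that explodes after a countdown and destroys itself once the explosion length elapses.
; Exploding disables physics and collision, toggles the placeholder sphere's visibility and adds a heavily scaled sphere component as the blast volume, with no effect logic attached.
; Tick tracks time since thrown so overlaps ignore the first half second, but hits only print debug text, as the second explode branch is unwired.
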(event OnComponentBeginOverlap(Collision)
  (params (OverlappedComponent :type Primitive%20Component%20Object%20Reference) (OtherActor :type Actor%20Object%20Reference) (OtherComp :type Primitive%20Component%20Object%20Reference) (OtherBodyIndex :type Integer) (bFromSweep :type Boolean) (SweepResult :type Hit%20Result%20Structure%20%28by%20ref%29))
  (if (>= (Variables|Default|GetTimeSinceThrown) 0.5)
    (Development|PrintText "Hit!")))

(event Custom|ExplodeBomb
  (bind _collision (Variables|Default|GetCollision))
  (Variables|Default|SetHasExploded true)
  (Physics|SetSimulatePhysics _collision false)
  (Collision|SetCollisionEnabled _collision "NoCollision")
  (Rendering|ToggleVisibility (Variables|Default|GetPlaceholderSphere) false)
  (AddComponent|AddSphereComponent false (Math|Transform|MakeTransform "0, 0, 0" "0, 0, 0" "75.000000,75.000000,75.000000"))
  (Development|PrintText "Exploded naturally")
  (Utilities|FlowControl|Delay (Variables|Default|GetExplosionLength))
  (Actor|DestroyActor))

(event Collision|EventActorBeginOverlap
  (params (OtherActor :type Actor%20Object%20Reference)))

(event EventTick
  (params (DeltaSeconds :type Float%20%28single-precision%29))
  (Variables|Default|SetTimeSinceThrown (+ (Variables|Default|GetTimeSinceThrown) DeltaSeconds)))

(event EventBeginPlay
  (Utilities|FlowControl|Delay (Variables|Default|GetBombCountdown))
  (if (not (Variables|Default|GetHasExploded))
    (CallFunction|ExplodeBomb)))

(fn ConstructionScript)