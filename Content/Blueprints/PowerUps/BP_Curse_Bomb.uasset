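; BP_Curse_Bomb is a thrown curse power-up bomb that explodes after a countdown or on overlapping a BP_Truck.
; Exploding disables collision and physics, toggles the placeholder sphere's visibility, adds a large sphere component, then destroys the actor after ExplosionLength.
; A HasExploded flag guards both triggers; no damage or effect is applied here.
; The overlap trigger requires TimeSinceThrown of at least 0.5, but Tick adds zero to that timer.
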(event OnComponentBeginOverlap(Collision)
  (params (OverlappedComponent :type Primitive%20Component%20Object%20Reference) (OtherActor :type Actor%20Object%20Reference) (OtherComp :type Primitive%20Component%20Object%20Reference) (OtherBodyIndex :type Integer) (bFromSweep :type Boolean) (SweepResult :type Hit%20Result%20Structure%20%28by%20ref%29))
  (if (>= (Variables|Default|GetTimeSinceThrown) 0.5)
    (Development|PrintText "Hit!")
    (Utilities|Casting|CastToBP_Truck OtherActor)
    (if (not (Variables|Default|GetHasExploded))
      (CallFunction|ExplodeBomb))))

(event Custom|ExplodeBomb
  (bind _placeholdersphere (Variables|Default|GetPlaceholderSphere))
  (bind _collision (Variables|Default|GetCollision))
  (Variables|Default|SetHasExploded true)
  (Physics|SetSimulatePhysics _collision false)
  (Collision|SetCollisionEnabled _collision "NoCollision")
  (Rendering|ToggleVisibility _placeholdersphere false)
  (AddComponent|AddSphereComponent true (Math|Transform|MakeTransform (Transformation|GetWorldLocation _placeholdersphere) "0, 0, 0" "75.000000,75.000000,75.000000"))
  (Development|PrintText "Exploded naturally")
  (Utilities|FlowControl|Delay (Variables|Default|GetExplosionLength))
  (Actor|DestroyActor))

(event EventBeginPlay
  (Utilities|FlowControl|Delay (Variables|Default|GetBombCountdown))
  (if (not (Variables|Default|GetHasExploded))
    (CallFunction|ExplodeBomb)))

(event Collision|EventActorBeginOverlap
  (params (OtherActor :type Actor%20Object%20Reference)))

(event EventTick
  (params (DeltaSeconds :type Float%20%28single-precision%29))
  (Variables|Default|SetTimeSinceThrown (+ (Variables|Default|GetTimeSinceThrown) 0.0)))

(fn ConstructionScript)