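; Test game mode for the truck game that registers joining players and relays lobby mode and level selections to the first player controller.
; PostLogin numbers each controller, stores it in the game instance and publishes player states to the game state.
; It binds truck health-change delegates on login, BeginPlay and pawn changes.
; The death handler is empty; old kill and timed player-start respawn logic remains disconnected for reference.
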(event Custom|UpdateLobby
  (bind _currentgamemode (Variables|Default|GetCurrentGameMode))
  (bind _asbp_truck_player_controller (Utilities|Casting|CastToBP_TruckPlayerController (Game|GetPlayerController 0)))
  (Default|UpdateGameMode _asbp_truck_player_controller _currentgamemode)
  (Development|PrintString (Utilities|String|EnumtoString _currentgamemode) true true "(R=0.259066,G=1.000000,B=0.168297,A=1.000000)"))

(event Custom|OnPlayerPawnChanged
  (params (OldPawn :type Pawn%20Object%20Reference) (NewPawn :type Pawn%20Object%20Reference))
  ;[0.15 0.15 0.15 0.5] Set-up for player starts
  (bind _asbp_truck (Utilities|Casting|CastToBP_Truck NewPawn))
  (CallFunction|OnKillandRespawn (Pawn|GetController _asbp_truck)))

(event Custom|Update%20maps
  (bind _asbp_truck_player_controller (Utilities|Casting|CastToBP_TruckPlayerController (Game|GetPlayerController 0)))
  (Default|UpdatelevelSelection _asbp_truck_player_controller (Variables|Default|GetSelctedLevelnName)))

(event EventBeginPlay
  (bind _asgs_gtdagame_state (Utilities|Casting|CastToGS_GTDAGameState (Game|GetGameState)))
  (Variables|/Game/Blueprints/Backend/GS_GTDAGameState.GS_GTDAGameState_C|SetGameMode _asgs_gtdagame_state "NewEnumerator1")
  (bind _asbp_truck_game_instance (Utilities|Casting|CastToBP_TruckGameInstance (Game|GetGameInstance)))
  (Variables|Default|SetAll_ConnectedControllers (Variables|/Game/Blueprints/Backend/BP_TruckGameInstance.BP_TruckGameInstance_C|GetPlayerControllers _asbp_truck_game_instance))
  (Utilities|FlowControl|Delay 2.0)
  (Development|PrintString (Utilities|String|ToString(Integer) (Utilities|Array|Length (Variables|Default|GetAll_ConnectedControllers))))
  (for _array_element (Variables|Default|GetAll_ConnectedControllers)
    (Pawn|BindEventtoOnPossessedPawnChanged _array_element (EventDispatchers|CreateEvent :!event Custom|OnPlayerPawnChanged))
    (CallFunction|OnKillandRespawn _array_element)))

(event EventPostLogin
  (params (NewPlayer :type Player%20Controller%20Object%20Reference))
  (bind _numplayer (Variables|Default|GetNumPlayer))
  ;[0.15 0.15 0.15 0.5] Set-up for player starts
  (Development|PrintString "onpostlogin")
  (bind _asgs_gtdagame_state (Utilities|Casting|CastToGS_GTDAGameState (Game|GetGameState))
    (:then
      (Math|Integer|IncrementInt (Variables|/Game/Blueprints/Backend/GS_GTDAGameState.GS_GTDAGameState_C|GetNumPlayers _asgs_gtdagame_state)
        (:%20%20
          (bind _asbp_truck_player_controller (Utilities|Casting|CastToBP_TruckPlayerController NewPlayer)
            (:then
              (bind _asbp_truck_player_state (Utilities|Casting|CastToBP_TruckPlayerState (Variables|/Script/Engine.Controller|GetPlayerState _asbp_truck_player_controller))
                (:then
                  (Utilities|Array|Add (Variables|Default|GetAllConnectedPlayerStates) _asbp_truck_player_state)
                  (Variables|/Game/Blueprints/Players/CustomTruck/BP_TruckPlayerController.BP_TruckPlayerController_C|SetPlayerNum _asbp_truck_player_controller _numplayer)
                  (Math|Integer|IncrementInt _numplayer
                    (:%20%20
                      (Utilities|Array|Add (Variables|Default|GetAll_ConnectedControllers) _asbp_truck_player_controller)
                      (bind _asbp_truck_game_instance (Utilities|Casting|CastToBP_TruckGameInstance (Game|GetGameInstance)))
                      (Utilities|Array|Add (Variables|/Game/Blueprints/Backend/BP_TruckGameInstance.BP_TruckGameInstance_C|GetPlayerControllers _asbp_truck_game_instance) _asbp_truck_player_controller)
                      (bind _asgs_gtdagame_state_2 (Utilities|Casting|CastToGS_GTDAGameState (Game|GetGameState))
                        (:then
                          (Variables|/Game/Blueprints/Backend/GS_GTDAGameState.GS_GTDAGameState_C|SetAllConnectedPlayers _asgs_gtdagame_state_2 (Variables|Default|GetAllConnectedPlayerStates))
                          (Development|PrintString "Playe set")
                          (for _array_element (Variables|Default|GetAll_ConnectedControllers)
                            (CallFunction|OnKillandRespawn _array_element)
                            (Pawn|BindEventtoOnPossessedPawnChanged _array_element (delegate Custom|OnPlayerPawnChanged))))
                        (:CastFailed
                          (Development|PrintString "GameState cast failed"))))))
                (:CastFailed
                  (Development|PrintString "Player State Fail"))))
            (:CastFailed
              (Development|PrintString "Player Cast fail" true true "(R=0.000000,G=0.660000,B=1.000000,A=1.000000)" 2e+01))))))
    (:CastFailed
      (Development|PrintString "Gamestate cast fail"))))

(event Custom|SetSelcectedGameMode
  (params (CurrentGameMode :type E_GameMode%20Enum :default "NewEnumerator1"))
  (Variables|Default|SetCurrentGameMode CurrentGameMode)
  (CallFunction|UpdateLobby))

(event Custom|OnKillAndRespawn
  (params (Controller :type Controller%20Object%20Reference))
  ;[0.15 0.15 0.15 0.5] Bind delegate to watch truck health changes
  (bind _asbp_truck_player_controller (Utilities|Casting|CastToBP_TruckPlayerController Controller))
  (Utilities|IsValid (Variables|/Game/Blueprints/Players/CustomTruck/BP_TruckPlayerController.BP_TruckPlayerController_C|GetTruck _asbp_truck_player_controller)
    (:Is%20Valid
      (EventDispatchers|BindEventtoOnHealthChange (Variables|/Game/Blueprints/Players/CustomTruck/BP_TruckPlayerController.BP_TruckPlayerController_C|GetTruck _asbp_truck_player_controller) (delegate Custom|CheckForPlayerDeath)))))

(event Custom|CheckForPlayerDeath
  (params (CurrentHealth :type Float%20%28double-precision%29) (MaxHealth :type Float%20%28double-precision%29) (TruckController :type BP%20Truck%20Player%20Controller%20Object%20Reference) (OtherActor :type Actor%20Object%20Reference)))

(event Custom|ParticlesOnAllClients
  (params (NewParam :type Niagara%20Component%20Object%20Reference)))

(event Custom|RespawnPlayer
  ;[0.15 0.15 0.15 0.5] Replaced but kept code here for reference
  (Default|ClientRPCEnd (stale Custom|CheckForPlayerDeath TruckController))
  (bind _returnvalue (Game|SpawnActorfromClass "/Game/Blueprints/Players/CustomTruck/BP_Truck.BP_Truck_C" (Transformation|GetActorTransform (Class|GameModeBase|FindPlayerStart (stale Custom|CheckForPlayerDeath TruckController) (Utilities|String|ToString(Integer) (Variables|/Game/Blueprints/Players/CustomTruck/BP_TruckPlayerController.BP_TruckPlayerController_C|GetPlayerNum (stale Custom|CheckForPlayerDeath TruckController))))) "AdjustIfPossibleButAlwaysSpawn" "MultiplyWithRoot" 0 0))
  (bind _asbp_truck_player_state (Utilities|Casting|CastToBP_TruckPlayerState (Variables|/Script/Engine.Controller|GetPlayerState (Game|GetPlayerController (Variables|/Game/Blueprints/Players/CustomTruck/BP_TruckPlayerController.BP_TruckPlayerController_C|GetPlayerNum (stale Custom|CheckForPlayerDeath TruckController))))))
  (Variables|/Game/Blueprints/Players/CustomTruck/BP_TruckPlayerState.BP_TruckPlayerState_C|SetBoostNum _asbp_truck_player_state 1e+02)
  (Pawn|Possess (stale Custom|CheckForPlayerDeath TruckController) _returnvalue))

(fn ConstructionScript)

(fn OnRepPlayerIsDead)

(fn OnRepDeadPlayerLocation
  (Niagara|SpawnSystematLocation "/Game/VFX/ParticleSystems/PS_Death_Explosion.PS_Death_Explosion" (Variables|Default|GetDeadPlayerLocation)))