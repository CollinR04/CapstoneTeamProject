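; Thrown chain bomb that explodes on a countdown or on hitting a BP_Truck after a short arming time.
; A truck hit temporarily lowers its MaxSpeed and shows its SlowdownChains ribbon.
; Exploding disables collision, hides the projectile and adds a sphere hitbox, with delayed destruction that outlasts the slowdown timer.
; Explosion effects toggle through replicate events that forward to all-client events.
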(event OnComponentBeginOverlap(Collision)
  (params (OverlappedComponent :type Primitive%20Component%20Object%20Reference) (OtherActor :type Actor%20Object%20Reference) (OtherComp :type Primitive%20Component%20Object%20Reference) (OtherBodyIndex :type Integer) (bFromSweep :type Boolean) (SweepResult :type Hit%20Result%20Structure%20%28by%20ref%29))
  (if (>= (Variables|Default|GetTimeSinceThrown) 0.5)
    (bind _asbp_truck (Utilities|Casting|CastToBP_Truck OtherActor))
    (if (Variables|Default|GetHasExploded)
      _
      (else
        (CallFunction|ExplodeBomb)))
    (Default|ReplicateRibbonActivate _asbp_truck (Variables|/Game/Blueprints/Players/CustomTruck/BP_Truck.BP_Truck_C|GetSlowdown%20Chains _asbp_truck))
    (Variables|/Game/Blueprints/Players/CustomTruck/BP_Truck.BP_Truck_C|SetMaxSpeed _asbp_truck 0.5)
    (Utilities|FlowControl|Delay 1e+01)
    (Variables|/Game/Blueprints/Players/CustomTruck/BP_Truck.BP_Truck_C|SetMaxSpeed _asbp_truck 1.0)
    (Default|ReplicateRibbonDeactivate _asbp_truck (Variables|/Game/Blueprints/Players/CustomTruck/BP_Truck.BP_Truck_C|GetSlowdown%20Chains _asbp_truck))))

(event Custom|ExplodeBomb
  (bind _collision (Variables|Default|GetCollision))
  (Variables|Default|SetHasExploded true)
  (Physics|SetSimulatePhysics _collision false)
  (Collision|SetCollisionEnabled _collision "NoCollision")
  (Rendering|ToggleVisibility (Actor|GetComponentsByClass "/Script/Engine.StaticMeshComponent") false)
  (Rendering|ToggleVisibility (Variables|Default|GetPS_Chain_Projectile_Aura) false)
  (bind _returnvalue (AddComponent|AddSphereComponent true (Math|Transform|MakeTransform (Transformation|GetWorldLocation (Variables|Default|GetBall)) "0, 0, 0" "75.000000,75.000000,75.000000")))
  (Variables|Default|SetExplosionHitbox _returnvalue)
  (CallFunction|ReplicateEffectActivate (Variables|Default|GetExplosion))
  (Utilities|FlowControl|Delay (Variables|Default|GetExplosionLength))
  (CallFunction|ReplicateEffectDeactivate (Variables|Default|GetExplosion))
  (Collision|SetCollisionEnabled (Variables|Default|GetExplosionHitbox) "NoCollision")
  (Utilities|FlowControl|Delay 12.0)
  (Actor|DestroyActor))

(event EventBeginPlay
  (Utilities|FlowControl|Delay (Variables|Default|GetBombCountdown))
  (if (not (Variables|Default|GetHasExploded))
    (CallFunction|ExplodeBomb)))

(event Collision|EventActorBeginOverlap
  (params (OtherActor :type Actor%20Object%20Reference)))

(event EventTick
  (params (DeltaSeconds :type Float%20%28single-precision%29))
  (Variables|Default|SetTimeSinceThrown (+ (Variables|Default|GetTimeSinceThrown) DeltaSeconds)))

(event Custom|ReplicateEffectDeactivate
  (params (Effect :type Actor%20Component%20Object%20Reference))
  (CallFunction|DeactivateonAllClients Effect))

(event Custom|DeactivateOnAllClients
  (params (Effect :type Actor%20Component%20Object%20Reference))
  (Components|Activation|Deactivate Effect))

(event Custom|ReplicateEffectActivate
  (params (Effect :type Actor%20Component%20Object%20Reference))
  (CallFunction|ActivateonAllClients Effect))

(event Custom|ActivateOnAllClients
  (params (Effect :type Actor%20Component%20Object%20Reference))
  (Components|Activation|SetActive Effect true false))

(fn ConstructionScript)